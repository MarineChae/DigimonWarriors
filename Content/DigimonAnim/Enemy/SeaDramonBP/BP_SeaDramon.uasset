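; SeaDramon enemy Blueprint, a ranged Digimon that attacks the player with ice sphere projectiles.
; BeginPlay configures the parent's montages, stats, attack range and skill cooldown, then writes skill availability to the AI blackboard.
; AttackStart and UseSkill each spawn a projectile at the head socket, aimed at the player pawn's current position.
; The skill variant flies faster and calls CoolDown after a successful spawn.
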(event Custom|AttackStart
  (CallFunction|SpawnAttackIceSpere))

(event Custom|UseSkill
  (CallFunction|SpawnSkillIceSpere))

(event EventBeginPlay
  (|CallParentFunction)
  (Variables|Default|SetHitMontage "/Game/DigimonAnim/Enemy/SeaDramon/AnimMontage_SeaDramonHit.AnimMontage_SeaDramonHit")
  (Variables|Default|SetAttack%20Montage "/Game/DigimonAnim/Enemy/SeaDramon/AnimMontage_SeadramonAttack.AnimMontage_SeadramonAttack")
  (Variables|Default|SetDie%20Montage "/Game/DigimonAnim/Enemy/SeaDramon/AnimMontage_SeaDramonDeath.AnimMontage_SeaDramonDeath")
  (Variables|Default|SetSkill%20Montage "/Game/DigimonAnim/Enemy/SeaDramon/AnimMOntage_SeaDramonSkill.AnimMOntage_SeaDramonSkill")
  (Variables|Default|SetAttackRange 8e+02)
  (Variables|Default|SetEXP 4e+02)
  (bind _output_get (Variables|Default|SetMax%20HP 2.5e+03))
  (Variables|Default|SetHP _output_get)
  (Variables|Default|SetSkillCoolDown 5.0)
  (bind _output_get_2 (Variables|Default|SetCanuseSkill true))
  (AI|Components|Blackboard|SetValueasBool (AI|GetBlackboard 0) (Variables|Default|GetCheckUseSKill) _output_get_2))

(event Collision|EventActorBeginOverlap
  (params (OtherActor :type Actor%20Object%20Reference)))

(event EventTick
  (params (DeltaSeconds :type Float%20%28single-precision%29))
  (|CallParentFunction DeltaSeconds) ; 지금 이 노드는 비활성 상태입니다. \n핀을 끌어서 다른 노드를 연결하면 활성화됩니다.
)

(fn ConstructionScript
  (|CallParentFunction))

(fn SpawnAttackIceSpere
  (bind _returnvalue (Game|GetPlayerController 0))
  (bind _mesh (Variables|Character|GetMesh))
  (bind _returnvalue_2 (Transformation|GetSocketLocation _mesh "HeadSkillSocket"))
  (bind _returnvalue_3 (Pawn|GetControlledPawn _returnvalue))
  (bind _returnvalue_4 (Transformation|GetActorLocation _returnvalue_3))
  (bind _returnvalue_5 (- _returnvalue_4 _returnvalue_2))
  (bind (_x _y _z) (Math|Vector|BreakVector _returnvalue_5))
  (bind _returnvalue_6 (Math|Vector|MakeVector _x _y _z))
  (bind _returnvalue_7 (Game|SpawnActorfromClass "/Game/DigimonAnim/Skill/BP_IceSpere.BP_IceSpere_C" (Math|Conversions|ToTransform(Vector) _returnvalue_2) "Undefined" "MultiplyWithRoot" self 0))
  (Utilities|IsValid _returnvalue_7
    (:Is%20Valid
      (Transformation|SetActorRotation _returnvalue_7 (Math|Conversions|RotationFromXVector _returnvalue_6))
      (bind _output_get (Variables|Default|SetProjectile _returnvalue_7))
      (Variables|/Script/Engine.MovementComponent|SetVelocity (Variables|/Game/DigimonAnim/Skill/BP_Projectile.BP_Projectile_C|GetProjectileMovement _output_get) (* (Math|Vector|Normalize _returnvalue_6) 3.5e+03)))))

(fn SpawnSkillIceSpere
  (bind _returnvalue (Game|GetPlayerController 0))
  (bind _mesh (Variables|Character|GetMesh))
  (bind _returnvalue_2 (Pawn|GetControlledPawn _returnvalue))
  (bind _returnvalue_3 (Transformation|GetSocketLocation _mesh "HeadSkillSocket"))
  (bind _returnvalue_4 (Transformation|GetActorLocation _returnvalue_2))
  (bind _returnvalue_5 (- _returnvalue_4 _returnvalue_3))
  (bind (_x _y _z) (Math|Vector|BreakVector _returnvalue_5))
  (bind _returnvalue_6 (Math|Vector|MakeVector _x _y _z))
  (bind _returnvalue_7 (Game|SpawnActorfromClass "/Game/DigimonAnim/Skill/BP_IceSpereSKill.BP_IceSpereSKill_C" (Math|Conversions|ToTransform(Vector) _returnvalue_3) "Undefined" "MultiplyWithRoot" self 0))
  (Utilities|IsValid _returnvalue_7
    (:Is%20Valid
      (Transformation|SetActorRotation _returnvalue_7 (Math|Conversions|RotationFromXVector _returnvalue_6))
      (bind _output_get (Variables|Default|SetProjectile _returnvalue_7))
      (Variables|/Script/Engine.MovementComponent|SetVelocity (Variables|/Game/DigimonAnim/Skill/BP_Projectile.BP_Projectile_C|GetProjectileMovement _output_get) (* (Math|Vector|Normalize _returnvalue_6) 5e+03))
      (CallFunction|CoolDown))))