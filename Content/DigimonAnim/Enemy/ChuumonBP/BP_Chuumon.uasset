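; Chuumon enemy Blueprint that attacks at range by throwing cheese projectiles.
; BeginPlay runs the parent logic, hides the held cheese mesh, and sets the hit, attack and death montages, EXP reward and attack range.
; PickCheese shows the mesh; ThrowCheese hides it and spawns an owned BP_Cheese at the hand socket location.
; The projectile's velocity follows the actor's forward vector at a fixed speed, with no target aiming.
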(event Custom|PickCheese
  (Development|SetHiddeninGame (Variables|Default|GetStaticMesh) false false))

(event Custom|ThrowCheese
  (Development|SetHiddeninGame (Variables|Default|GetStaticMesh) true false)
  (bind _returnvalue (Game|SpawnActorfromClass "/Game/DigimonAnim/Skill/BP_Cheese.BP_Cheese_C" (Math|Conversions|ToTransform(Vector) (Transformation|GetSocketLocation (Variables|Default|GetStaticMesh) "J_hand_R소켓")) "Undefined" "MultiplyWithRoot" self 0))
  (Utilities|IsValid _returnvalue
    (:Is%20Valid
      (bind _output_get (Variables|Default|SetProjectile _returnvalue))
      (Variables|/Script/Engine.MovementComponent|SetVelocity (Variables|/Game/DigimonAnim/Skill/BP_Projectile.BP_Projectile_C|GetProjectileMovement _output_get) (* (Math|Vector|Normalize (Math|Vector|GetForwardVector (Transformation|GetActorRotation))) 1.5e+03)))))

(event EventBeginPlay
  (|CallParentFunction)
  (Development|SetHiddeninGame (Variables|Default|GetStaticMesh) true false)
  (Variables|Default|SetHitMontage "/Game/DigimonAnim/Enemy/Chuumon/AnimMontage_ChumonHit.AnimMontage_ChumonHit")
  (Variables|Default|SetAttack%20Montage "/Game/DigimonAnim/Enemy/Chuumon/AnimMontage_ChuumonAttack.AnimMontage_ChuumonAttack")
  (Variables|Default|SetDie%20Montage "/Game/DigimonAnim/Enemy/Chuumon/AnimMontage_ChumonDie.AnimMontage_ChumonDie")
  (Variables|Default|SetEXP 15.0)
  (Variables|Default|SetAttackRange 7e+02))

(fn ConstructionScript
  (|CallParentFunction))