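; Base enemy character that handles combat, health, death and granting EXP to BP_AgumonGamemode.
; Tick tracks flattened distance and direction to the player, keeping a spawned HP bar actor facing along it.
; Damage updates health, shows a boss widget when a portrait is set, and triggers death or, on heavy hits, a stagger montage.
; Attack, death and skill-cooldown states feed Blackboard keys, while skill and attack-collision-end events are empty hooks.
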(event Custom|AttackCollisionEnd
  ;[1 1 1] Projectile
)

(event Custom|UseSKill
  ;[1 1 1] Projectile
)

(event Custom|Save%20Dis&Dir
  (bind _returnvalue (Game|GetPlayerController 0))
  (bind _returnvalue_2 (Transformation|GetActorLocation))
  (bind _returnvalue_3 (Pawn|GetControlledPawn _returnvalue))
  (bind _returnvalue_4 (Transformation|GetActorLocation _returnvalue_3))
  (bind _returnvalue_5 (- _returnvalue_4 _returnvalue_2))
  (bind (_x _y) (Math|Vector|BreakVector _returnvalue_5))
  (bind _returnvalue_6 (Math|Vector|MakeVector _x _y 0.0))
  ;[1 1 1] Dis&Dir to Player
  (Variables|Default|SetDistance%20To%20Player (Math|Vector|VectorLength _returnvalue_6))
  (Variables|Default|SetDirection%20To%20Player (Math|Vector|Normalize _returnvalue_6)))

(event Custom|AttackEnd
  ;[1 1 1] Attack
  (bind _output_get (Variables|Default|SetIsAttack false))
  (CallFunction|BlackBoardAttack _output_get))

(event Custom|CoolDown
  (bind _output_get (Variables|Default|SetCanuseSkill false))
  (AI|Components|Blackboard|SetValueasBool (AI|GetBlackboard 0) (Variables|Default|GetCheckUseSKill) _output_get)
  (bind _output_get_2 (Variables|Default|SetRemainTime 0.0))
  (if (<= _output_get_2 (Variables|Default|GetSkillCoolDown)) :!label _label
    (Utilities|FlowControl|Delay 0.1)
    (Variables|Default|SetRemainTime (+ _output_get_2 0.1))
    (goto _label)
    (else
      (bind _output_get_3 (Variables|Default|SetCanuseSkill true))
      (AI|Components|Blackboard|SetValueasBool (AI|GetBlackboard 0) (Variables|Default|GetCheckUseSKill) _output_get_3))))

(event Custom|Attack
  ;[1 1 1] Attack
  (if (not (Variables|Default|GetIsHit))
    (Animation|PlayAnimMontage (Variables|Default|GetAttack%20Montage) 1.0 "None")
    (bind _output_get (Variables|Default|SetIsAttack true))
    (CallFunction|BlackBoardAttack _output_get)))

(event EventTick
  (params (DeltaSeconds :type Float%20%28single-precision%29))
  (bind _hpwidget (Variables|Default|GetHPWidget))
  (CallFunction|SaveDis&Dir)
  (Utilities|IsValid _hpwidget
    (:Is%20Valid
      (Default|UpdateLocation _hpwidget (Transformation|GetWorldLocation (Variables|Default|GetHpBar)))
      (Default|UpdateRotate _hpwidget (Math|Conversions|RotationFromXVector (Variables|Default|GetDirection%20to%20Player))))))

(event Game|Damage|EventAnyDamage
  (params (Damage :type Float%20%28single-precision%29) (DamageType :type Damage%20Type%20Object%20Reference) (InstigatedBy :type Controller%20Object%20Reference) (DamageCauser :type Actor%20Object%20Reference))
  (bind _bosswidget (Variables|Default|GetBossWidget))
  ;[1 1 1] Damage Taken
  (Variables|Default|SetIsHit true)
  (CallFunction|PlayHitSound)
  (CallFunction|CreateHPWidget)
  (if (not (Variables|Default|GetIs%20Dying))
    (bind _output_get (Variables|Default|SetHP (- (Variables|Default|GetHP) Damage)))
    (Default|UpdateHpBar (Variables|Default|GetHPWidget) _output_get (Variables|Default|GetMax%20HP))
    (if (<= _output_get 0.0)
      (AI|Components|Blackboard|SetValueasBool (AI|GetBlackboard 0) (Variables|Default|GetCheckDead) (<= _output_get 0.0))
      (CallFunction|EnemyDie)
      (bind _asbp_agumon_gamemode (Utilities|Casting|CastToBP_AgumonGamemode (Game|GetGameMode)))
      (Default|GetExp _asbp_agumon_gamemode (Variables|Default|GetEXP))
      (Utilities|IsValid _bosswidget
        (:Is%20Valid
          (Widget|RemovefromParent _bosswidget)))
      (else
        (Variables|Default|SetIsHit false)
        (if (Variables|Default|GetIsAttack)
          _
          (else
            (Transformation|SetActorRotation (Math|Conversions|RotationFromXVector (Variables|Default|GetDirection%20to%20Player)))))
        (if (>= (/ Damage (Variables|Default|GetMax%20HP)) 0.1)
          (CallFunction|AttackCollisionEnd)
          (bind _returnvalue (Animation|PlayAnimMontage (Variables|Default|GetHitMontage) 1.0 "None"))
          (Utilities|FlowControl|Delay _returnvalue)
          (bind _output_get_2 (Variables|Default|SetIsAttack false))
          (CallFunction|BlackBoardAttack _output_get_2))))))

(event EventBeginPlay
  ;[1 1 1] Init
  (bind _returnvalue (Game|SpawnActorfromClass "/Game/DigimonAnim/UI/BP_HPWidget.BP_HPWidget_C" (Math|Transform|MakeTransform (Transformation|GetWorldLocation (Variables|Default|GetHpBar))) "Undefined" "MultiplyWithRoot" 0 0))
  (Variables|Default|SetHPWidget _returnvalue)
  (Audio|Components|Audio|Stop (Variables|Default|GethardHit)))

(fn ConstructionScript)

(fn UpdateWalkSpeed
  (params (NewWalkSpeed :type Float%20%28double-precision%29))
  (Variables|/Script/Engine.CharacterMovementComponent|SetMaxWalkSpeed (Variables|Character|GetCharacterMovement) NewWalkSpeed))

(fn FireDamage
  (bind _output_get (Variables|Default|SetHP (- (Variables|Default|GetHP) 2e+01)))
  (Default|UpdateHpBar (Variables|Default|GetHPWidget) _output_get (Variables|Default|GetMax%20HP))
  (if (<= _output_get 0.0)
    (bind _output_get_2 (Variables|Default|SetAttack%20Montage "/Game/DigimonAnim/Enemy/Chuumon/AnimMontage_ChumonDie.AnimMontage_ChumonDie"))
    (Animation|PlayAnimMontage _output_get_2 1.0 "None")
    (Variables|Default|SetIs%20Dying true)
    (Collision|SetCollisionEnabled (Variables|Collision|GetCapsuleComponent) "NoCollision")
    (Collision|SetCollisionEnabled (Variables|Character|GetMesh) "NoCollision")
    (Actor|DestroyActor (Variables|Default|GetHPWidget))))

(fn Endfire
  (Utilities|Time|ClearandInvalidateTimerbyHandle (Variables|Default|GetTimer)))

(fn EnemyDie
  (Animation|PlayAnimMontage (Variables|Default|GetDie%20Montage) 1.0 "None")
  (Variables|Default|SetIs%20Dying true)
  (Collision|SetCollisionEnabled (Variables|Collision|GetCapsuleComponent) "NoCollision")
  (Collision|SetCollisionEnabled (Variables|Character|GetMesh) "NoCollision")
  (CallFunction|AttackCollisionEnd)
  (Actor|DestroyActor (Variables|Default|GetHPWidget)))

(fn CheckHit
  (params (other :type Actor%20Object%20Reference))
  (bind _self self)
  (if (not (== other self))
    (if (Actor|ActorHasTag other "Player")
      (if (Variables|/Script/Engine.Actor|GetbCanBeDamaged other)
        (Game|Damage|ApplyDamage other (Variables|Default|GetBase%20Damage) (AI|GetAIController _self) _self)))))

(fn BlackBoardAttack
  (params (Attack? :type Boolean))
  (AI|Components|Blackboard|SetValueasBool (AI|GetBlackboard 0) (LocalVariables|GetIsAttack?) Attack?))

(fn CreateHPWidget
  (if (not (Variables|Default|GetWidgetIsCreate?))
    (Utilities|IsValid (Variables|Default|GetPortarit)
      (:Is%20Valid
        (bind _returnvalue (UserInterface|CreateWidget "/Game/DigimonAnim/UI/WBP_BossHP.WBP_BossHP_C"))
        (Variables|Default|SetBossWidget _returnvalue)
        (UserInterface|Viewport|AddtoViewport _returnvalue 0)
        (Variables|Default|SetWidgetIsCreate? true)))))

(fn PlayHitSound
  (Audio|Components|Audio|Play (Variables|Default|GethardHit) 0.0))