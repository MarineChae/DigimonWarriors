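; Nanomon enemy Blueprint, a child of a shared enemy class that sets its own montages, attack range, EXP reward, HP and base damage on BeginPlay.
; Melee hits come from left and right hand colliders, switched on separately by collision events and off together when the attack ends.
; Hand overlaps pass the other actor to CheckHit, and the EnemyDie override disables both colliders after the parent logic.
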(event OnComponentBeginOverlap(LeftHand)
  (params (OverlappedComponent :type Primitive%20Component%20Object%20Reference) (OtherActor :type Actor%20Object%20Reference) (OtherComp :type Primitive%20Component%20Object%20Reference) (OtherBodyIndex :type Integer) (bFromSweep :type Boolean) (SweepResult :type Hit%20Result%20Structure%20%28by%20ref%29))
  (CallFunction|CheckHit OtherActor))

(event OnComponentBeginOverlap(RightHand)
  (params (OverlappedComponent :type Primitive%20Component%20Object%20Reference) (OtherActor :type Actor%20Object%20Reference) (OtherComp :type Primitive%20Component%20Object%20Reference) (OtherBodyIndex :type Integer) (bFromSweep :type Boolean) (SweepResult :type Hit%20Result%20Structure%20%28by%20ref%29))
  (CallFunction|CheckHit OtherActor))

(event Custom|AttackCollisionEnd
  (Collision|SetCollisionEnabled (Variables|Default|GetLeftHand) "NoCollision")
  (Collision|SetCollisionEnabled (Variables|Default|GetRightHand) "NoCollision"))

(event Custom|CollisionStart
  (Collision|SetCollisionEnabled (Variables|Default|GetRightHand) "QueryAndPhysics"))

(event Custom|CollisionLeft
  (Collision|SetCollisionEnabled (Variables|Default|GetLeftHand) "QueryAndPhysics"))

(event EventBeginPlay
  (|CallParentFunction)
  (Variables|Default|SetHitMontage "/Game/DigimonAnim/Enemy/Nanomon/AnimMontage_NanomonHit.AnimMontage_NanomonHit")
  (Variables|Default|SetAttack%20Montage "/Game/DigimonAnim/Enemy/Nanomon/AnimMontage_NanomonAtack.AnimMontage_NanomonAtack")
  (Variables|Default|SetDie%20Montage "/Game/DigimonAnim/Enemy/Nanomon/AnimMontage_NanomonDie.AnimMontage_NanomonDie")
  (Variables|Default|SetAttackRange 7e+02)
  (Variables|Default|SetEXP 1e+02)
  (bind _output_get (Variables|Default|SetMax%20HP 1.4e+03))
  (Variables|Default|SetHP _output_get)
  (Variables|Default|SetBase%20Damage 8e+01))

(event Collision|EventActorBeginOverlap
  (params (OtherActor :type Actor%20Object%20Reference)))

(event EventTick
  (params (DeltaSeconds :type Float%20%28single-precision%29))
  (|CallParentFunction DeltaSeconds) ; 지금 이 노드는 비활성 상태입니다. \n핀을 끌어서 다른 노드를 연결하면 활성화됩니다.
)

(fn ConstructionScript
  (|CallParentFunction))

(fn EnemyDie
  (|CallParentFunction)
  (Collision|SetCollisionEnabled (Variables|Default|GetLeftHand) "NoCollision")
  (Collision|SetCollisionEnabled (Variables|Default|GetRightHand) "NoCollision"))