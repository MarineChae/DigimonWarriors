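; AI controller for a boss enemy that starts a behavior tree on possession and tracks the player through AI perception.
; Sensing a Player-tagged actor cancels the forget timer and writes line of sight and target to the blackboard.
; Any other perception update starts that timer, which clears both keys when it expires.
; An older distance-based Idle/Move chase state machine remains in the graph but never runs.
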(event OnTargetPerceptionUpdated(AIPerception)
  (params (Actor :type Actor%20Object%20Reference) (Stimulus :type AI%20Stimulus%20Structure))
  (bind _blackboard (Variables|Default|GetBlackboard))
  ;[1 1 1] 코멘트
  (if (and (Actor|ActorHasTag Actor "Player") (Utilities|Struct|BreakAIStimulus Stimulus))
    (Utilities|Time|ClearandInvalidateTimerbyHandle (Variables|Default|GetEnemyTimer))
    (AI|Components|Blackboard|SetValueasBool _blackboard (Variables|Default|GetHasLineSight) true)
    (AI|Components|Blackboard|SetValueasObject _blackboard (Variables|Default|GetEnemyActor) Actor)
    (else
      (bind _returnvalue (Utilities|Time|SetTimerbyEvent (delegate Custom|StartEnemyTimer) (Variables|Default|GetLine%20Of%20Sight%20Timer)))
      (Variables|Default|SetEnemyTimer _returnvalue))))

(event Custom|Save%20Disd&Dir
  (bind _returnvalue (Game|GetPlayerCharacter 0))
  (bind _returnvalue_2 (Pawn|GetControlledPawn))
  (bind _returnvalue_3 (Transformation|GetActorLocation _returnvalue))
  (bind _returnvalue_4 (Transformation|GetActorLocation _returnvalue_2))
  (bind _returnvalue_5 (- _returnvalue_3 _returnvalue_4))
  (bind (_x _y) (Math|Vector|BreakVector _returnvalue_5))
  (bind _returnvalue_6 (Math|Vector|MakeVector _x _y 0.0))
  ;[1 1 1] Dis&Dir to Player
  (Variables|Default|SetDistance%20To%20Player (Math|Vector|VectorLength _returnvalue_6))
  (Variables|Default|SetDirection%20To%20Player (Math|Vector|Normalize _returnvalue_6)))

(event Custom|StartEnemyTimer
  (bind _blackboard (Variables|Default|GetBlackboard))
  ;[1 1 1] 코멘트
  (AI|Components|Blackboard|SetValueasBool _blackboard (Variables|Default|GetHasLineSight) false)
  (AI|Components|Blackboard|SetValueasObject _blackboard (Variables|Default|GetEnemyActor) 0))

(event EventPossess
  (params (PossessedPawn :type Pawn%20Object%20Reference))
  (AI|RunBehaviorTree "/Game/DigimonAnim/Enemy/BossTree/BT_AIBTBoss.BT_AIBTBoss"))

(fn ConstructionScript)