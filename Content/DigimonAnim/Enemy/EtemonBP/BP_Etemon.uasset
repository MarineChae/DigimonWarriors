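; Etemon enemy character that sets its own montages, stats, portrait and skill cooldown on the parent enemy logic.
; Left and right hand colliders toggle through events, feed hit checks on overlap and switch off on death.
; Its skill spawns a gravity-free, non-colliding projectile at a socket and starts cooldown; ShotSkill later launches it forward with gravity and collision.
; BreakWall explodes and destroys all spinning rune stone actors.
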(event OnComponentBeginOverlap(LeftHand)
  (params (OverlappedComponent :type Primitive%20Component%20Object%20Reference) (OtherActor :type Actor%20Object%20Reference) (OtherComp :type Primitive%20Component%20Object%20Reference) (OtherBodyIndex :type Integer) (bFromSweep :type Boolean) (SweepResult :type Hit%20Result%20Structure%20%28by%20ref%29))
  (CallFunction|CheckHit OtherActor))

(event OnComponentBeginOverlap(RightHand)
  (params (OverlappedComponent :type Primitive%20Component%20Object%20Reference) (OtherActor :type Actor%20Object%20Reference) (OtherComp :type Primitive%20Component%20Object%20Reference) (OtherBodyIndex :type Integer) (bFromSweep :type Boolean) (SweepResult :type Hit%20Result%20Structure%20%28by%20ref%29))
  (CallFunction|CheckHit OtherActor))

(event Custom|AttackCollisionEnd
  (Collision|SetCollisionEnabled (Variables|Default|GetLeftHand) "NoCollision")
  (Collision|SetCollisionEnabled (Variables|Default|GetRightHand) "NoCollision"))

(event Custom|CollisionRight
  (Collision|SetCollisionEnabled (Variables|Default|GetRightHand) "QueryAndPhysics"))

(event Custom|CollisionLeft
  (Collision|SetCollisionEnabled (Variables|Default|GetLeftHand) "QueryAndPhysics"))

(event Custom|BreakWall
  (bind _outactors (Actor|GetAllActorsOfClass "/Game/DreamscapeSeries/DreamscapeTower/Blueprints/BP_SpiningRuneStonesBreak.BP_SpiningRuneStonesBreak_C"))
  (for _array_element _outactors
    (Effects|SpawnEmitteratLocation "/Game/FXVarietyPack/Particles/P_ky_explosion.P_ky_explosion" (Transformation|GetActorLocation _array_element) "0, 0, 0" "3.000000,3.000000,3.000000")
    (Audio|PlaySoundatLocation "/Game/Sound/Explosion01.Explosion01" (Transformation|GetActorLocation _array_element) "0, 0, 0" 0.05 1.0 0.0 0 0 0 0)
    (Actor|DestroyActor _array_element)))

(event Custom|ShotSkill
  (bind _as_bp_projectile (Variables|Default|GetAs%20BP%20Projectile))
  (bind _projectilemovement (Variables|/Game/DigimonAnim/Skill/BP_Projectile.BP_Projectile_C|GetProjectileMovement _as_bp_projectile))
  (Utilities|IsValid _as_bp_projectile
    (:Is%20Valid
      (Variables|/Script/Engine.ProjectileMovementComponent|SetProjectileGravityScale _projectilemovement 5.0)
      (Variables|/Script/Engine.MovementComponent|SetVelocity _projectilemovement (* (Math|Vector|Normalize (Math|Vector|GetForwardVector (Transformation|GetActorRotation))) (Variables|Default|GetProjectile%20Speed)))
      (Collision|SetCollisionEnabled (Variables|/Game/DigimonAnim/Skill/BP_Projectile.BP_Projectile_C|GetSphere _as_bp_projectile) "QueryAndPhysics"))))

(event EventBeginPlay
  (|CallParentFunction)
  (Variables|Default|SetHitMontage "/Game/DigimonAnim/Enemy/Etemon/AnimMontage_EtemonHit.AnimMontage_EtemonHit")
  (Variables|Default|SetAttack%20Montage "/Game/DigimonAnim/Enemy/Etemon/AnimMonate_EtemonAttack.AnimMonate_EtemonAttack")
  (Variables|Default|SetDie%20Montage "/Game/DigimonAnim/Enemy/Etemon/AnimMontage_EtemonDeath.AnimMontage_EtemonDeath")
  (Variables|Default|SetSkill%20Montage "/Game/DigimonAnim/Enemy/Etemon/AnimMontage_EtemonSkill.AnimMontage_EtemonSkill")
  (Variables|Default|SetBase%20Damage 4e+01)
  (Variables|Default|SetPortarit "/Game/DigimonAnim/Enemy/EtemonBP/Portrait_Type_D.Portrait_Type_D")
  (Variables|Default|SetAttackRange 5e+02)
  (Variables|Default|SetEXP 1e+03)
  (bind _output_get (Variables|Default|SetMax%20HP 6e+03))
  (Variables|Default|SetHP _output_get)
  (Variables|Default|SetSkillCoolDown 8.0)
  (bind _output_get_2 (Variables|Default|SetCanuseSkill true))
  (AI|Components|Blackboard|SetValueasBool (AI|GetBlackboard 0) (Variables|Default|GetCheckUseSKill) _output_get_2)
  (Rendering|SetActorHiddenInGame (Variables|Default|GetHPWidget) true))

(event Collision|EventActorBeginOverlap
  (params (OtherActor :type Actor%20Object%20Reference)))

(event EventTick
  (params (DeltaSeconds :type Float%20%28single-precision%29))
  (|CallParentFunction DeltaSeconds) ; 지금 이 노드는 비활성 상태입니다. \n핀을 끌어서 다른 노드를 연결하면 활성화됩니다.
)

(event EventUseSKill
  (CallFunction|SpawnSkill))

(fn ConstructionScript
  (|CallParentFunction))

(fn SpawnSkill
  (bind _returnvalue (Game|SpawnActorfromClass "/Game/DigimonAnim/Skill/BP_EtemonSkill.BP_EtemonSkill_C" (Math|Conversions|ToTransform(Vector) (Transformation|GetSocketLocation (Variables|Character|GetMesh) "SKillSocket")) "AlwaysSpawn" "MultiplyWithRoot" 0 0))
  (bind _asbp_projectile (Utilities|Casting|CastToBP_Projectile _returnvalue))
  (Transformation|SetActorRotation _returnvalue (Transformation|GetActorRotation))
  (Collision|SetCollisionEnabled (Variables|/Game/DigimonAnim/Skill/BP_Projectile.BP_Projectile_C|GetSphere _asbp_projectile) "NoCollision")
  (bind _output_get (Variables|Default|SetAs%20BP%20Projectile _asbp_projectile))
  (Variables|/Script/Engine.ProjectileMovementComponent|SetProjectileGravityScale (Variables|/Game/DigimonAnim/Skill/BP_Projectile.BP_Projectile_C|GetProjectileMovement _output_get) 0.0)
  (CallFunction|CoolDown))

(fn EnemyDie
  (|CallParentFunction)
  (Collision|SetCollisionEnabled (Variables|Default|GetLeftHand) "NoCollision")
  (Collision|SetCollisionEnabled (Variables|Default|GetRightHand) "NoCollision"))