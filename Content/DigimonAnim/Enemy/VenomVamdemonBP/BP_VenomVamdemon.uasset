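; VenomVamdemon enemy Blueprint that sets up montages, stats and portrait on its parent enemy logic, flags skill readiness in the Blackboard and hides its HP widget.
; Its skill fires a BP_VenomBeam from the mesh's SkillSocket toward a player position cached by GetLocation, then starts the cooldown; SkillEnd destroys the beam.
; Melee attacks toggle right-hand collision through start and end events, passing overlapped actors to CheckHit.
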(event OnComponentBeginOverlap(RightHand)
  (params (OverlappedComponent :type Primitive%20Component%20Object%20Reference) (OtherActor :type Actor%20Object%20Reference) (OtherComp :type Primitive%20Component%20Object%20Reference) (OtherBodyIndex :type Integer) (bFromSweep :type Boolean) (SweepResult :type Hit%20Result%20Structure%20%28by%20ref%29))
  (CallFunction|CheckHit OtherActor))

(event Custom|AttackCollisionStart
  (Collision|SetCollisionEnabled (Variables|Default|GetRightHand) "QueryAndPhysics"))

(event Custom|AttackCollisionEnd
  (Collision|SetCollisionEnabled (Variables|Default|GetRightHand) "NoCollision"))

(event Custom|SkillEnd
  (Actor|DestroyActor (Variables|Default|GetLazer)))

(event Custom|GetLocation
  (Variables|Default|SetPlayerPos (Transformation|GetActorLocation (Pawn|GetControlledPawn (Game|GetPlayerController 0)))))

(event EventBeginPlay
  (|CallParentFunction)
  (Variables|Default|SetHitMontage "/Game/DigimonAnim/Enemy/VenomVamdemon/AnimMontage_VenomHit.AnimMontage_VenomHit")
  (Variables|Default|SetAttack%20Montage "/Game/DigimonAnim/Enemy/VenomVamdemon/AnimMontage_VenomAttack.AnimMontage_VenomAttack")
  (Variables|Default|SetDie%20Montage "/Game/DigimonAnim/Enemy/VenomVamdemon/AnimMontage_VenomDie.AnimMontage_VenomDie")
  (Variables|Default|SetSkill%20Montage "/Game/DigimonAnim/Enemy/VenomVamdemon/AnimMontage_VenomSkill.AnimMontage_VenomSkill")
  (Variables|Default|SetBase%20Damage 1.5e+02)
  (Variables|Default|SetPortarit "/Game/DigimonAnim/Enemy/VenomVamdemonBP/Portrait_Type_A.Portrait_Type_A")
  (Variables|Default|SetAttackRange 7e+02)
  (bind _output_get (Variables|Default|SetMax%20HP 1.5e+04))
  (Variables|Default|SetHP _output_get)
  (Variables|Default|SetSkillCoolDown 7.0)
  (bind _output_get_2 (Variables|Default|SetCanuseSkill true))
  (AI|Components|Blackboard|SetValueasBool (AI|GetBlackboard 0) (Variables|Default|GetCheckUseSKill) _output_get_2)
  (Rendering|SetActorHiddenInGame (Variables|Default|GetHPWidget) true))

(event Collision|EventActorBeginOverlap
  (params (OtherActor :type Actor%20Object%20Reference)))

(event EventTick
  (params (DeltaSeconds :type Float%20%28single-precision%29))
  (|CallParentFunction DeltaSeconds) ; 지금 이 노드는 비활성 상태입니다. \n핀을 끌어서 다른 노드를 연결하면 활성화됩니다.
)

(event EventUseSKill
  (bind _playerpos (Variables|Default|GetPlayerPos))
  (bind _mesh (Variables|Character|GetMesh))
  (bind _returnvalue (Transformation|GetSocketLocation _mesh "SkillSocket"))
  (bind _returnvalue_2 (- _playerpos _returnvalue))
  (bind (_x _y _z) (Math|Vector|BreakVector _returnvalue_2))
  (bind _returnvalue_3 (Game|SpawnActorfromClass "/Game/DigimonAnim/Skill/BP_VenomBeam.BP_VenomBeam_C" (Math|Transform|MakeTransform _returnvalue (Math|Conversions|RotationFromXVector (Math|Vector|MakeVector _x _y _z))) "Undefined" "MultiplyWithRoot" self 0))
  (bind _output_get (Variables|Default|SetLazer _returnvalue_3))
  (Utilities|IsValid _output_get
    (:Is%20Valid
      (CallFunction|CoolDown))))

(fn ConstructionScript
  (|CallParentFunction))