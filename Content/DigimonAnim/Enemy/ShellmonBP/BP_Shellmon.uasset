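; Shellmon enemy Blueprint that sets its montages, portrait and combat stats on BeginPlay and hides its HP widget.
; Its skill spawns a BP_WaterShot at the head socket, aims and launches it at the player's current position, then starts cooldown.
; A blackboard flag is initialized to mark the skill usable.
; Melee attack events toggle LeftHand collision, and overlaps pass the other actor to CheckHit.
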(event OnComponentBeginOverlap(LeftHand)
  (params (OverlappedComponent :type Primitive%20Component%20Object%20Reference) (OtherActor :type Actor%20Object%20Reference) (OtherComp :type Primitive%20Component%20Object%20Reference) (OtherBodyIndex :type Integer) (bFromSweep :type Boolean) (SweepResult :type Hit%20Result%20Structure%20%28by%20ref%29))
  (CallFunction|CheckHit OtherActor))

(event Custom|AttackCollisionStart
  (Collision|SetCollisionEnabled (Variables|Default|GetLeftHand) "QueryAndPhysics"))

(event Custom|AttackCollisionEnd
  (Collision|SetCollisionEnabled (Variables|Default|GetLeftHand) "NoCollision"))

(event Custom|UseSkill
  (bind _returnvalue (Game|GetPlayerController 0))
  (bind _mesh (Variables|Character|GetMesh))
  (bind _returnvalue_2 (Transformation|GetSocketLocation _mesh "HeadSkillSocket"))
  (bind _returnvalue_3 (Pawn|GetControlledPawn _returnvalue))
  (bind _returnvalue_4 (Transformation|GetActorLocation _returnvalue_3))
  (bind _returnvalue_5 (- _returnvalue_4 _returnvalue_2))
  (bind (_x _y _z) (Math|Vector|BreakVector _returnvalue_5))
  (bind _returnvalue_6 (Math|Vector|MakeVector _x _y _z))
  (bind _returnvalue_7 (Game|SpawnActorfromClass "/Game/DigimonAnim/Skill/BP_WaterShot.BP_WaterShot_C" (Math|Conversions|ToTransform(Vector) _returnvalue_2) "Undefined" "MultiplyWithRoot" self 0))
  (Utilities|IsValid _returnvalue_7
    (:Is%20Valid
      (Transformation|SetActorRotation _returnvalue_7 (Math|Conversions|RotationFromXVector _returnvalue_6))
      (bind _output_get (Variables|Default|SetProjectile _returnvalue_7))
      (Variables|/Script/Engine.MovementComponent|SetVelocity (Variables|/Game/DigimonAnim/Skill/BP_Projectile.BP_Projectile_C|GetProjectileMovement _output_get) (* (Math|Vector|Normalize _returnvalue_6) 1.5e+03))
      (CallFunction|CoolDown))))

(event EventBeginPlay
  (|CallParentFunction)
  (Variables|Default|SetHitMontage "/Game/DigimonAnim/Enemy/Shellmon/AnimMontage_shellmonHit.AnimMontage_shellmonHit")
  (Variables|Default|SetAttack%20Montage "/Game/DigimonAnim/Enemy/Shellmon/AnimMontage_ShellmonAttack.AnimMontage_ShellmonAttack")
  (Variables|Default|SetDie%20Montage "/Game/DigimonAnim/Enemy/Shellmon/AnimMontage_ShellmonDie.AnimMontage_ShellmonDie")
  (Variables|Default|SetSkill%20Montage "/Game/DigimonAnim/Enemy/Shellmon/AnimMontage_ShellmonSkill.AnimMontage_ShellmonSkill")
  (Variables|Default|SetPortarit "/Game/DigimonAnim/Enemy/ShellmonBP/Portrait_Type_D.Portrait_Type_D")
  (Variables|Default|SetAttackRange 6.5e+02)
  (Variables|Default|SetEXP 4e+02)
  (bind _output_get (Variables|Default|SetMax%20HP 2.5e+03))
  (Variables|Default|SetHP _output_get)
  (Variables|Default|SetSkillCoolDown 5.0)
  (bind _output_get_2 (Variables|Default|SetCanuseSkill true))
  (AI|Components|Blackboard|SetValueasBool (AI|GetBlackboard 0) (Variables|Default|GetCheckUseSKill) _output_get_2)
  (Rendering|SetActorHiddenInGame (Variables|Default|GetHPWidget) true))

(event Collision|EventActorBeginOverlap
  (params (OtherActor :type Actor%20Object%20Reference)))

(event EventTick
  (params (DeltaSeconds :type Float%20%28single-precision%29))
  (|CallParentFunction DeltaSeconds) ; 지금 이 노드는 비활성 상태입니다. \n핀을 끌어서 다른 노드를 연결하면 활성화됩니다.
)

(fn ConstructionScript
  (|CallParentFunction))