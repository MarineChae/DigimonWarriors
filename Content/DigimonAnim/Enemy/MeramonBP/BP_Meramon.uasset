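; BP_Meramon is the Meramon enemy Blueprint, a child that fills in stats and montages for its parent enemy class.
; BeginPlay calls the parent, then assigns hit, attack and death montages plus attack range, damage, experience and health.
; AttackCollisionStart and AttackCollisionEnd events toggle collision on the RightHand component, limiting when attacks can connect.
; RightHand overlaps pass the other actor to CheckHit.
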(event OnComponentBeginOverlap(RightHand)
  (params (OverlappedComponent :type Primitive%20Component%20Object%20Reference) (OtherActor :type Actor%20Object%20Reference) (OtherComp :type Primitive%20Component%20Object%20Reference) (OtherBodyIndex :type Integer) (bFromSweep :type Boolean) (SweepResult :type Hit%20Result%20Structure%20%28by%20ref%29))
  (CallFunction|CheckHit OtherActor))

(event Custom|AttackCollisionStart
  (Collision|SetCollisionEnabled (Variables|Default|GetRightHand) "QueryAndPhysics"))

(event Custom|AttackCollisionEnd
  (Collision|SetCollisionEnabled (Variables|Default|GetRightHand) "NoCollision"))

(event EventBeginPlay
  (|CallParentFunction)
  (Variables|Default|SetHitMontage "/Game/DigimonAnim/Enemy/Meramon/AnimMontage_MeramonHit.AnimMontage_MeramonHit")
  (Variables|Default|SetAttack%20Montage "/Game/DigimonAnim/Enemy/Meramon/AnimMontage_MeramonAttack.AnimMontage_MeramonAttack")
  (Variables|Default|SetDie%20Montage "/Game/DigimonAnim/Enemy/Meramon/AnimMontage_MeramonDie.AnimMontage_MeramonDie")
  (Variables|Default|SetAttackRange 3.5e+02)
  (Variables|Default|SetEXP 4e+01)
  (Variables|Default|SetBase%20Damage 2e+01)
  (bind _output_get (Variables|Default|SetMax%20HP 8e+02))
  (Variables|Default|SetHP _output_get))

(event Collision|EventActorBeginOverlap
  (params (OtherActor :type Actor%20Object%20Reference)))

(event EventTick
  (params (DeltaSeconds :type Float%20%28single-precision%29))
  (|CallParentFunction DeltaSeconds) ; 지금 이 노드는 비활성 상태입니다. \n핀을 끌어서 다른 노드를 연결하면 활성화됩니다.
)

(fn ConstructionScript
  (|CallParentFunction))