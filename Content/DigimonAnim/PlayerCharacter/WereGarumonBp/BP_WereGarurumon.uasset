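; Playable WereGarurumon character Blueprint, a melee evolution stage between Garurumon and MetalGarurumon.
; BeginPlay fills inherited variables with its montages, skill cooldown, widget, portrait, evolution links and evolution cutscene media.
; Attacks and the skill toggle left and right hand collision, whose overlaps feed CheckHit; WarGreymon-named events handle the attack window.
; While ActiveHeraldry is set, Tick calls EquipHeraldry at player level 5+ if a slot holds FriendShipTag.
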(event OnComponentBeginOverlap(LeftHand)
  (params (OverlappedComponent :type Primitive%20Component%20Object%20Reference) (OtherActor :type Actor%20Object%20Reference) (OtherComp :type Primitive%20Component%20Object%20Reference) (OtherBodyIndex :type Integer) (bFromSweep :type Boolean) (SweepResult :type Hit%20Result%20Structure%20%28by%20ref%29))
  (CallFunction|CheckHit OtherActor))

(event OnComponentBeginOverlap(RightHand)
  (params (OverlappedComponent :type Primitive%20Component%20Object%20Reference) (OtherActor :type Actor%20Object%20Reference) (OtherComp :type Primitive%20Component%20Object%20Reference) (OtherBodyIndex :type Integer) (bFromSweep :type Boolean) (SweepResult :type Hit%20Result%20Structure%20%28by%20ref%29))
  (CallFunction|CheckHit OtherActor))

(event Custom|WarGreymonAtttackcollsionStart
  (Collision|SetCollisionEnabled (Variables|Default|GetRightHand) "QueryAndPhysics"))

(event Custom|WarGreymonAtttackcollsionEnd
  (Collision|SetCollisionEnabled (Variables|Default|GetRightHand) "NoCollision")
  (Collision|SetCollisionEnabled (Variables|Default|GetLeftHand) "NoCollision"))

(event EventBeginPlay
  (|CallParentFunction)
  (Variables|Default|SetAttack%20Montage "/Game/DigimonAnim/PlayerCharacter/Weregarumon/AnimMontage_WereGarurumonAttack.AnimMontage_WereGarurumonAttack")
  (Variables|Default|SetSKillMontage "/Game/DigimonAnim/PlayerCharacter/Weregarumon/AnimMontage_WereGarurumon.AnimMontage_WereGarurumon")
  (Variables|Default|SetSpawnprojectile 0)
  (Variables|Default|SetPrevEvolutionName "/Game/DigimonAnim/PlayerCharacter/GarumonBP/BP_Garumon.BP_Garumon_C")
  (Variables|Default|SetEvoMontage "/Game/DigimonAnim/PlayerCharacter/Weregarumon/AnimMontage_WereGaruAvo.AnimMontage_WereGaruAvo")
  (bind _output_get (Variables|Default|SetSkillColldown 5.0))
  (Variables|Default|SetRemainTime _output_get)
  (Variables|Default|SetWidget%20Class "/Game/DigimonAnim/UI/SkillIcon/WBP_Weregaru.WBP_Weregaru_C")
  (Variables|Default|SetNextEvolutionName "/Game/DigimonAnim/PlayerCharacter/MetalGarumonBP/BP_MetalGarumon.BP_MetalGarumon_C")
  (Variables|Default|SetLevelUpEmitter "/Game/InfinityBladeEffects/Effects/FX_Mobile/ICE/P_levelUp_Ice.P_levelUp_Ice")
  (Variables|Default|SetEvoScene "/Game/DigimonAnim/NewMediaPlayer.NewMediaPlayer")
  (Variables|Default|SetMedia%20Source "/Game/Movies/metalgaru2.metalgaru2")
  (Variables|Default|SetPortrait "/Game/DigimonAnim/PlayerCharacter/WereGarumonBp/werw.werw")
  (Variables|Default|SetDie%20Montage "/Game/DigimonAnim/PlayerCharacter/Weregarumon/AM_WereGaruDie.AM_WereGaruDie"))

(event EventTick
  (params (DeltaSeconds :type Float%20%28single-precision%29))
  (bind _playerslot (Variables|Default|GetPlayerSlot))
  (if (Variables|Default|GetActiveHeraldry)
    (bind _asbp_new_gabumon_gamemode (Utilities|Casting|CastToBP_NewGabumonGamemode (Game|GetGameMode)))
    (if (>= (Variables|/Game/ThirdPerson/Blueprints/BP_AgumonGamemode.BP_AgumonGamemode_C|GetPlayer%20Level _asbp_new_gabumon_gamemode) 5)
      (bind _array_index (Utilities|Array|ForEachLoopwithBreak _playerslot)
        (:LoopBody
          (if (== (.rowname (Utilities|Struct|BreakS_Slot (Utilities|Array|Get(acopy) _playerslot _array_index))) "FriendShipTag")
            (CallFunction|EquipHeraldry)))))))

(event EventUseSkill
  (Collision|SetCollisionEnabled (Variables|Default|GetRightHand) "QueryAndPhysics")
  (Collision|SetCollisionEnabled (Variables|Default|GetLeftHand) "QueryAndPhysics")
  (CallFunction|CoolDown))

(fn ConstructionScript
  (|CallParentFunction))