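; BP_MetalGarumon is the playable MetalGarurumon Digimon character, evolved from WereGarurumon with no further evolution set.
; BeginPlay fills in parent-class data such as montages, stats, skill cooldown, portrait and widget.
; Melee attack events toggle RightHand collision, and its overlaps go to CheckHit.
; UseSkill spawns a BP_GaruMissile at a hatch socket, launches it along player 0's pawn facing, and starts the cooldown.
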(event OnComponentBeginOverlap(RightHand)
  (params (OverlappedComponent :type Primitive%20Component%20Object%20Reference) (OtherActor :type Actor%20Object%20Reference) (OtherComp :type Primitive%20Component%20Object%20Reference) (OtherBodyIndex :type Integer) (bFromSweep :type Boolean) (SweepResult :type Hit%20Result%20Structure%20%28by%20ref%29))
  (CallFunction|CheckHit OtherActor))

(event Custom|AttackCollsionStart
  (Collision|SetCollisionEnabled (Variables|Default|GetRightHand) "QueryAndPhysics"))

(event Custom|AttackCollsionEnd
  (Collision|SetCollisionEnabled (Variables|Default|GetRightHand) "NoCollision"))

(event EventBeginPlay
  (|CallParentFunction)
  (Variables|Default|SetAttack%20Montage "/Game/DigimonAnim/PlayerCharacter/MetalGarumon/AnimMontage_MetalgarumonAttack.AnimMontage_MetalgarumonAttack")
  (Variables|Default|SetSKillMontage "/Game/DigimonAnim/PlayerCharacter/MetalGarumon/AnimMontage_MetalGarumonSkill.AnimMontage_MetalGarumonSkill")
  (Variables|Default|SetSpawnprojectile "/Game/DigimonAnim/Skill/BP_GaruMissile.BP_GaruMissile_C")
  (Variables|Default|SetPrevEvolutionName "/Game/DigimonAnim/PlayerCharacter/WereGarumonBp/BP_WereGarurumon.BP_WereGarurumon_C")
  (Variables|Default|SetEvoMontage "/Game/DigimonAnim/PlayerCharacter/MetalGarumon/AnimMontage_MetalGaruEvo.AnimMontage_MetalGaruEvo")
  (bind _output_get (Variables|Default|SetSkillColldown 8.0))
  (Variables|Default|SetRemainTime _output_get)
  (Variables|Default|SetClearMontage "/Game/DigimonAnim/PlayerCharacter/MetalGarumon/AnimMontage_MetalGaru_Clear.AnimMontage_MetalGaru_Clear")
  (Variables|Default|SetNextEvolutionName 0)
  (Variables|Default|SetProjectileSpeed 2.5e+03)
  (Variables|Default|SetClearMontage "/Game/DigimonAnim/PlayerCharacter/MetalGarumon/AnimMontage_MetalGaru_Clear.AnimMontage_MetalGaru_Clear")
  (Variables|Default|SetDie%20Montage "/Game/DigimonAnim/PlayerCharacter/MetalGarumon/AnimMontage_MetalGaruDie.AnimMontage_MetalGaruDie")
  (Variables|Default|SetLevelUpEmitter "/Game/InfinityBladeEffects/Effects/FX_Mobile/ICE/P_levelUp_Ice.P_levelUp_Ice")
  (Variables|Default|SetPortrait "/Game/DigimonAnim/PlayerCharacter/MetalGarumonBP/Portrait_Type_A.Portrait_Type_A")
  (Variables|Default|SetWidget%20Class "/Game/DigimonAnim/UI/SkillIcon/WBP_Metalgaru.WBP_Metalgaru_C")
  (Variables|Default|SetBase%20Damage 8e+02))

(event EventUseSkill
  (CallFunction|SpawnMissile "Hatch_R_Dum")
  (CallFunction|CoolDown))

(fn ConstructionScript
  (|CallParentFunction))

(fn SpawnMissile
  (params (SocketName :type Name))
  (bind _returnvalue (Game|GetPlayerController 0))
  (bind _returnvalue_2 (Pawn|GetControlledPawn _returnvalue))
  (bind _returnvalue_3 (Transformation|GetActorRotation _returnvalue_2))
  (bind _returnvalue_4 (Game|SpawnActorfromClass "/Game/DigimonAnim/Skill/BP_GaruMissile.BP_GaruMissile_C" (Math|Conversions|ToTransform(Vector) (Transformation|GetSocketLocation (Variables|Character|GetMesh) SocketName)) "AlwaysSpawn" "MultiplyWithRoot" 0 0))
  (bind _asbp_projectile (Utilities|Casting|CastToBP_Projectile _returnvalue_4))
  (Transformation|SetActorRotation _returnvalue_4 _returnvalue_3)
  (bind _output_get (Variables|Default|SetProjectile _asbp_projectile))
  (Variables|/Script/Engine.MovementComponent|SetVelocity (Variables|/Game/DigimonAnim/Skill/BP_Projectile.BP_Projectile_C|GetProjectileMovement _output_get) (* (Math|Vector|Normalize (Math|Vector|GetForwardVector _returnvalue_3)) (Variables|Default|GetProjectileSpeed))))