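; Omegamon player character Blueprint, a final evolution stage that configures its parent's montages, projectile, damage and evolution links on BeginPlay.
; Melee events toggle left-hand collision, overlaps feed CheckHit, and NextAttack advances a montage-section combo.
; The Garuru Cannon fires in two phases: charging spawns a zero-gravity projectile at a mesh socket, then the shot event enables its collision, restores partial gravity and launches it along the character's forward vector.
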(event OnComponentBeginOverlap(LeftHand)
  (params (OverlappedComponent :type Primitive%20Component%20Object%20Reference) (OtherActor :type Actor%20Object%20Reference) (OtherComp :type Primitive%20Component%20Object%20Reference) (OtherBodyIndex :type Integer) (bFromSweep :type Boolean) (SweepResult :type Hit%20Result%20Structure%20%28by%20ref%29))
  (CallFunction|CheckHit OtherActor))

(event Custom|AttackCollsionEnd
  (Collision|SetCollisionEnabled (Variables|Default|GetLeftHand) "NoCollision"))

(event Custom|AttackCollsionStart
  (Collision|SetCollisionEnabled (Variables|Default|GetLeftHand) "QueryAndPhysics"))

(event Custom|ChargingCanon
  (CallFunction|UseGaruruCanon))

(event Custom|Next%20Attack
  (if (Variables|Default|GetCanNextAttack)
    (Variables|Default|SetCanNextAttack false)
    (bind _result (Math|Integer|IncrementInt (Variables|Default|GetComboCount))
      (:%20%20
        (bind _output_get (Variables|Default|SetComboCount _result))
        (switch int _output_get
          (:1
            (Animation|PlayAnimMontage "/Game/DigimonAnim/PlayerCharacter/OmegamonBP/test/NewAnimMontage.NewAnimMontage" 1.0 "NextAttack")))))))

(event Custom|ShotGarurucanon
  (bind _projectile (Variables|Default|GetProjectile))
  (bind _projectilemovement (Variables|/Game/DigimonAnim/Skill/BP_Projectile.BP_Projectile_C|GetProjectileMovement _projectile))
  (Utilities|IsValid _projectile
    (:Is%20Valid
      (Collision|SetCollisionEnabled (Variables|/Game/DigimonAnim/Skill/BP_Projectile.BP_Projectile_C|GetSphere _projectile) "QueryAndPhysics")
      (Utilities|IsValid _projectile
        (:Is%20Valid
          (Variables|/Script/Engine.ProjectileMovementComponent|SetProjectileGravityScale _projectilemovement 0.5)
          (Variables|/Script/Engine.MovementComponent|SetVelocity _projectilemovement (* (Math|Vector|Normalize (Math|Vector|GetForwardVector (Transformation|GetActorRotation))) (Variables|Default|GetProjectileSpeed))))))))

(event EventBeginPlay
  (|CallParentFunction)
  (Variables|Default|SetAttack%20Montage "/Game/DigimonAnim/PlayerCharacter/OmegamonBP/test/NewAnimMontage.NewAnimMontage")
  (Variables|Default|SetSKillMontage "/Game/DigimonAnim/PlayerCharacter/OmegamonBP/test/NewAnimMontage.NewAnimMontage")
  (Variables|Default|SetSpawnprojectile "/Game/DigimonAnim/Skill/BP_GaiaForce.BP_GaiaForce_C")
  (Variables|Default|SetPrevEvolutionName "/Game/DigimonAnim/PlayerCharacter/MetalGreymonBP/BP_MetalGreymon.BP_MetalGreymon_C")
  (Variables|Default|SetNextEvolutionName 0)
  (Variables|Default|SetIn%20Socket%20Name "GaiaForceSocket")
  (Variables|Default|SetProjectileSpeed 3e+03)
  (Variables|Default|SetBase%20Damage 1e+03))

(event Collision|EventActorBeginOverlap
  (params (OtherActor :type Actor%20Object%20Reference)))

(event EventTick
  (params (DeltaSeconds :type Float%20%28single-precision%29)))

(fn ConstructionScript
  (|CallParentFunction))

(fn UseGaruruCanon
  (bind _returnvalue (Game|SpawnActorfromClass "/Game/DigimonAnim/Skill/BP_GaruruCanon.BP_GaruruCanon_C" (Math|Conversions|ToTransform(Vector) (Transformation|GetSocketLocation (Variables|Character|GetMesh) "GruruCanon")) "AlwaysSpawn" "MultiplyWithRoot" 0 0))
  (bind _asbp_projectile (Utilities|Casting|CastToBP_Projectile _returnvalue))
  (Transformation|SetActorRotation _returnvalue (Transformation|GetActorRotation (Pawn|GetControlledPawn (Game|GetPlayerController 0))))
  (bind _output_get (Variables|Default|SetProjectile _asbp_projectile))
  (Variables|/Script/Engine.ProjectileMovementComponent|SetProjectileGravityScale (Variables|/Game/DigimonAnim/Skill/BP_Projectile.BP_Projectile_C|GetProjectileMovement _output_get) 0.0))