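; BP_Garumon is the playable Garumon character, the evolution stage between Gabumon and WereGarurumon.
; BeginPlay fills inherited settings for montages, stats, UI and evolution links.
; Attack events toggle Head collision for hit checks, while UseSkill spawns blue fire at the head socket, matches pawn rotation and starts cooldown.
; While ActiveHeraldry is set, Tick equips heraldry if player level is at least five and a slot holds FriendShipTag.
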(event OnComponentBeginOverlap(Head)
  (params (OverlappedComponent :type Primitive%20Component%20Object%20Reference) (OtherActor :type Actor%20Object%20Reference) (OtherComp :type Primitive%20Component%20Object%20Reference) (OtherBodyIndex :type Integer) (bFromSweep :type Boolean) (SweepResult :type Hit%20Result%20Structure%20%28by%20ref%29))
  (CallFunction|CheckHit OtherActor))

(event Custom|AttackCollsionStart
  (Collision|SetCollisionEnabled (Variables|Default|GetHead) "QueryAndPhysics"))

(event Custom|AttackCollsionEnd
  (Collision|SetCollisionEnabled (Variables|Default|GetHead) "NoCollision"))

(event Custom|EndSkill
  (bind _skill (Variables|Default|GetSkill))
  (Utilities|IsValid _skill
    (:Is%20Valid
      (Actor|DestroyActor _skill))))

(event EventBeginPlay
  (|CallParentFunction)
  (Variables|Default|SetAttack%20Montage "/Game/DigimonAnim/PlayerCharacter/Garumon/AnimMontage_GarumonAttack.AnimMontage_GarumonAttack")
  (Variables|Default|SetSKillMontage "/Game/DigimonAnim/PlayerCharacter/Garumon/AnimMontage_GarumonSkil.AnimMontage_GarumonSkil")
  (Variables|Default|SetSpawnprojectile "/Game/DigimonAnim/Skill/BP_BlueFire.BP_BlueFire_C")
  (Variables|Default|SetPrevEvolutionName "/Game/DigimonAnim/PlayerCharacter/GabumonBP/BP_Gabumon.BP_Gabumon_C")
  (Variables|Default|SetEvoMontage "/Game/DigimonAnim/PlayerCharacter/Garumon/AnimMontage_GarumonEvo.AnimMontage_GarumonEvo")
  (bind _output_get (Variables|Default|SetSkillColldown 5.0))
  (Variables|Default|SetRemainTime _output_get)
  (Variables|Default|SetNextEvolutionName "/Game/DigimonAnim/PlayerCharacter/WereGarumonBp/BP_WereGarurumon.BP_WereGarurumon_C")
  (Variables|Default|SetIn%20Socket%20Name "HeadSocket")
  (Variables|Default|SetWidget%20Class "/Game/DigimonAnim/UI/SkillIcon/WBP_Garumon.WBP_Garumon_C")
  (Variables|Default|SetLevelUpEmitter "/Game/InfinityBladeEffects/Effects/FX_Mobile/ICE/P_levelUp_Ice.P_levelUp_Ice")
  (Variables|Default|SetPortrait "/Game/DigimonAnim/PlayerCharacter/GarumonBP/Portrait_Type_D.Portrait_Type_D")
  (Variables|Default|SetBase%20Damage 4e+02)
  (Variables|Default|SetDie%20Montage "/Game/DigimonAnim/PlayerCharacter/Garumon/AM_GarumonDie.AM_GarumonDie"))

(event EventTick
  (params (DeltaSeconds :type Float%20%28single-precision%29))
  (bind _playerslot (Variables|Default|GetPlayerSlot))
  (if (Variables|Default|GetActiveHeraldry)
    (bind _asbp_new_gabumon_gamemode (Utilities|Casting|CastToBP_NewGabumonGamemode (Game|GetGameMode)))
    (if (>= (Variables|/Game/ThirdPerson/Blueprints/BP_AgumonGamemode.BP_AgumonGamemode_C|GetPlayer%20Level _asbp_new_gabumon_gamemode) 5)
      (bind _array_index (Utilities|Array|ForEachLoopwithBreak _playerslot)
        (:LoopBody
          (if (== (.rowname (Utilities|Struct|BreakS_Slot (Utilities|Array|Get(acopy) _playerslot _array_index))) "FriendShipTag")
            (CallFunction|EquipHeraldry)))))))

(event EventUseSkill
  (bind _returnvalue (Game|SpawnActorfromClass (Variables|Default|GetSpawnprojectile) (Math|Conversions|ToTransform(Vector) (Transformation|GetSocketLocation (Variables|Character|GetMesh) (Variables|Default|GetIn%20Socket%20Name))) "AlwaysSpawn" "MultiplyWithRoot" 0 0))
  (bind _output_get (Variables|Default|SetSkill _returnvalue))
  (Transformation|SetActorRotation _output_get (Transformation|GetActorRotation (Game|Player|GetPlayerPawn 0)))
  (CallFunction|CoolDown))

(fn ConstructionScript
  (|CallParentFunction))