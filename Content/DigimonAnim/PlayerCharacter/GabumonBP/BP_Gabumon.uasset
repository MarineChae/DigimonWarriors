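; BP_Gabumon is the playable Gabumon character, configuring its parent with montages, widget, stats and Garumon as its next evolution.
; Attack collision events toggle LeftHand collision, and its overlaps feed CheckHit for melee hits.
; UseSkill spawns a BP_BlueFire projectile at the HeadFire socket, aligns it to player pawn rotation and starts the cooldown.
; EndSkill destroys the spawned skill actor after a validity check.
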(event OnComponentBeginOverlap(LeftHand)
  (params (OverlappedComponent :type Primitive%20Component%20Object%20Reference) (OtherActor :type Actor%20Object%20Reference) (OtherComp :type Primitive%20Component%20Object%20Reference) (OtherBodyIndex :type Integer) (bFromSweep :type Boolean) (SweepResult :type Hit%20Result%20Structure%20%28by%20ref%29))
  (CallFunction|CheckHit OtherActor))

(event Custom|AttackCollsionStart
  (Collision|SetCollisionEnabled (Variables|Default|GetLeftHand) "QueryAndPhysics"))

(event Custom|AttackCollsionEnd
  (Collision|SetCollisionEnabled (Variables|Default|GetLeftHand) "NoCollision"))

(event Custom|EndSkill
  (Utilities|IsValid 0
    (:Is%20Valid
      (Actor|DestroyActor (Variables|Default|GetSkill)))))

(event EventBeginPlay
  (Variables|Default|SetWidget%20Class "/Game/DigimonAnim/UI/SkillIcon/WBP_Gabumon.WBP_Gabumon_C")
  (|CallParentFunction)
  (Variables|Default|SetAttack%20Montage "/Game/DigimonAnim/PlayerCharacter/Gabumon/AnimMontage_GabumonAttack.AnimMontage_GabumonAttack")
  (Variables|Default|SetSKillMontage "/Game/DigimonAnim/PlayerCharacter/Gabumon/AnimMontage_GabumonSkill.AnimMontage_GabumonSkill")
  (Variables|Default|SetSpawnprojectile "/Game/DigimonAnim/Skill/BP_BlueFire.BP_BlueFire_C")
  (Variables|Default|SetPrevEvolutionName 0)
  (bind _output_get (Variables|Default|SetSkillColldown 3.0))
  (Variables|Default|SetRemainTime _output_get)
  (Variables|Default|SetNextEvolutionName "/Game/DigimonAnim/PlayerCharacter/GarumonBP/BP_Garumon.BP_Garumon_C")
  (Variables|Default|SetIn%20Socket%20Name "HeadFire")
  (Variables|Default|SetProjectileSpeed 1.5e+03)
  (Variables|Default|SetLevelUpEmitter "/Game/InfinityBladeEffects/Effects/FX_Mobile/ICE/P_levelUp_Ice.P_levelUp_Ice")
  (Variables|Default|SetPortrait "/Game/DigimonAnim/PlayerCharacter/GabumonBP/Portrait_Type_D.Portrait_Type_D")
  (Variables|Default|SetDie%20Montage "/Game/DigimonAnim/PlayerCharacter/Gabumon/AnimMontage_GubumonDie.AnimMontage_GubumonDie")
  (Variables|Default|SetBase%20Damage 2e+02))

(event EventUseSkill
  (bind _returnvalue (Game|SpawnActorfromClass (Variables|Default|GetSpawnprojectile) (Math|Conversions|ToTransform(Vector) (Transformation|GetSocketLocation (Variables|Character|GetMesh) (Variables|Default|GetIn%20Socket%20Name))) "AlwaysSpawn" "MultiplyWithRoot" 0 0))
  (bind _output_get (Variables|Default|SetSkill _returnvalue))
  (Transformation|SetActorRotation _output_get (Transformation|GetActorRotation (Game|Player|GetPlayerPawn 0)))
  (CallFunction|CoolDown))

(fn ConstructionScript
  (|CallParentFunction))