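; WarGreymon player character, the last stage in its evolution line after MetalGreymon, with claw melee and the Gaia Force skill.
; BeginPlay fills inherited variables with its montages, stats, widget and evolution links.
; UseSkill spawns an inert Gaia Force at a mesh socket and starts cooldown; ShotGaiaForce later enables its collision and gravity and launches it along pawn facing.
; Attack events toggle both hand colliders, whose overlaps call CheckHit.
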(event OnComponentBeginOverlap(RightHand)
  (params (OverlappedComponent :type Primitive%20Component%20Object%20Reference) (OtherActor :type Actor%20Object%20Reference) (OtherComp :type Primitive%20Component%20Object%20Reference) (OtherBodyIndex :type Integer) (bFromSweep :type Boolean) (SweepResult :type Hit%20Result%20Structure%20%28by%20ref%29))
  (CallFunction|CheckHit OtherActor))

(event OnComponentBeginOverlap(LeftHand)
  (params (OverlappedComponent :type Primitive%20Component%20Object%20Reference) (OtherActor :type Actor%20Object%20Reference) (OtherComp :type Primitive%20Component%20Object%20Reference) (OtherBodyIndex :type Integer) (bFromSweep :type Boolean) (SweepResult :type Hit%20Result%20Structure%20%28by%20ref%29))
  (CallFunction|CheckHit OtherActor))

(event Custom|WarGreymonAtttackcollsionStart
  (Collision|SetCollisionEnabled (Variables|Default|GetLeftHand) "QueryAndPhysics")
  (Collision|SetCollisionEnabled (Variables|Default|GetRightHand) "QueryAndPhysics"))

(event Custom|WarGreymonAtttackcollsionEnd
  (Collision|SetCollisionEnabled (Variables|Default|GetLeftHand) "NoCollision")
  (Collision|SetCollisionEnabled (Variables|Default|GetRightHand) "NoCollision"))

(event Custom|ShotGaiaForce
  (bind _as_bp_projectile (Variables|Default|GetAs%20BP%20Projectile))
  (bind _projectilemovement (Variables|/Game/DigimonAnim/Skill/BP_Projectile.BP_Projectile_C|GetProjectileMovement _as_bp_projectile))
  (Utilities|IsValid _as_bp_projectile
    (:Is%20Valid
      (Variables|/Script/Engine.ProjectileMovementComponent|SetProjectileGravityScale _projectilemovement 1e+01)
      (Variables|/Script/Engine.MovementComponent|SetVelocity _projectilemovement (* (Math|Vector|Normalize (Math|Vector|GetForwardVector (Transformation|GetActorRotation (Pawn|GetControlledPawn (Game|GetPlayerController 0))))) (Variables|Default|GetProjectileSpeed)))
      (Collision|SetCollisionEnabled (Variables|/Game/DigimonAnim/Skill/BP_Projectile.BP_Projectile_C|GetSphere _as_bp_projectile) "QueryAndPhysics"))))

(event EventBeginPlay
  (|CallParentFunction)
  (Variables|Default|SetAttack%20Montage "/Game/DigimonAnim/PlayerCharacter/WarGreymon/AnimMontage_WargreymonAttack.AnimMontage_WargreymonAttack")
  (Variables|Default|SetSKillMontage "/Game/DigimonAnim/PlayerCharacter/WarGreymon/AnimMontage_WarGreymonSkill.AnimMontage_WarGreymonSkill")
  (Variables|Default|SetSpawnprojectile "/Game/DigimonAnim/Skill/BP_GaiaForce.BP_GaiaForce_C")
  (Variables|Default|SetPrevEvolutionName "/Game/DigimonAnim/PlayerCharacter/MetalGreymonBP/BP_MetalGreymon.BP_MetalGreymon_C")
  (bind _output_get (Variables|Default|SetSkillColldown 8.0))
  (Variables|Default|SetRemainTime _output_get)
  (Variables|Default|SetEvoMontage "/Game/DigimonAnim/PlayerCharacter/WarGreymon/AnimMontage_WarGreyEvo.AnimMontage_WarGreyEvo")
  (Variables|Default|SetDie%20Montage "/Game/DigimonAnim/PlayerCharacter/WarGreymon/AnimMontage_WargreyDie.AnimMontage_WargreyDie")
  (Variables|Default|SetNextEvolutionName 0)
  (Variables|Default|SetIn%20Socket%20Name "GaiaForceSocket")
  (Variables|Default|SetProjectileSpeed 3e+03)
  (Variables|Default|SetPortrait "/Game/DigimonAnim/PlayerCharacter/WarGreymonBP/Portrait_Type_A.Portrait_Type_A")
  (Variables|Default|SetLevelUpEmitter "/Game/InfinityBladeEffects/Effects/FX_Mobile/Fire/P_levelUp_Fire.P_levelUp_Fire")
  (Variables|Default|SetWidget%20Class "/Game/DigimonAnim/UI/SkillIcon/WBP_WarGrey.WBP_WarGrey_C")
  (Variables|Default|SetBase%20Damage 4e+02)
  (Variables|Default|SetClearMontage "/Game/DigimonAnim/PlayerCharacter/WarGreymon/AnimMontate_WarGreyClear.AnimMontate_WarGreyClear")
  (Audio|Components|Audio|Stop (Variables|Default|GetAudio)))

(event EventUseSkill
  (bind _returnvalue (Game|SpawnActorfromClass (Variables|Default|GetSpawnprojectile) (Math|Conversions|ToTransform(Vector) (Transformation|GetSocketLocation (Variables|Character|GetMesh) (Variables|Default|GetIn%20Socket%20Name))) "AlwaysSpawn" "MultiplyWithRoot" 0 0))
  (bind _asbp_projectile (Utilities|Casting|CastToBP_Projectile _returnvalue))
  (Transformation|SetActorRotation _returnvalue (Transformation|GetActorRotation (Pawn|GetControlledPawn (Game|GetPlayerController 0))))
  (Collision|SetCollisionEnabled (Variables|/Game/DigimonAnim/Skill/BP_Projectile.BP_Projectile_C|GetSphere _asbp_projectile) "NoCollision")
  (bind _output_get (Variables|Default|SetAs%20BP%20Projectile _asbp_projectile))
  (Variables|/Script/Engine.ProjectileMovementComponent|SetProjectileGravityScale (Variables|/Game/DigimonAnim/Skill/BP_Projectile.BP_Projectile_C|GetProjectileMovement _output_get) 0.0)
  (CallFunction|CoolDown))

(fn ConstructionScript
  (|CallParentFunction))

(fn GrowUpSize
  (params (NewParam :type Actor%20Object%20Reference))
  (Transformation|SetActorScale3D NewParam (* (Transformation|GetActorScale3D NewParam) 1.2)))