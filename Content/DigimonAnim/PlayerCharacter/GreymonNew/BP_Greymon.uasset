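; BP_Greymon is the playable Greymon character, the evolution stage between Agumon and MetalGreymon, built on a shared parent class.
; BeginPlay fills inherited settings: montages, MegaFire projectile, evolution links, cooldown, damage and UI.
; Attack events toggle the Tail collider, whose overlaps feed CheckHit.
; While ActiveHeraldry is set, Tick polls player level and inventory slots, calling EquipHeraldry for a CourageTag at level 5 or above.
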(event OnComponentBeginOverlap(Tail)
  (params (OverlappedComponent :type Primitive%20Component%20Object%20Reference) (OtherActor :type Actor%20Object%20Reference) (OtherComp :type Primitive%20Component%20Object%20Reference) (OtherBodyIndex :type Integer) (bFromSweep :type Boolean) (SweepResult :type Hit%20Result%20Structure%20%28by%20ref%29))
  (CallFunction|CheckHit OtherActor))

(event EventBeginPlay
  (|CallParentFunction)
  (Variables|Default|SetAttack%20Montage "/Game/DigimonAnim/PlayerCharacter/Greymon/AnimMontage_GreymonAttack.AnimMontage_GreymonAttack")
  (Variables|Default|SetSKillMontage "/Game/DigimonAnim/PlayerCharacter/Greymon/AnimMontage_Greyskill.AnimMontage_Greyskill")
  (Variables|Default|SetSpawnprojectile "/Game/DigimonAnim/Skill/BP_MegaFire.BP_MegaFire_C")
  (Variables|Default|SetPrevEvolutionName "/Game/DigimonAnim/PlayerCharacter/AgumonNew/BP_Agumon.BP_Agumon_C")
  (Variables|Default|SetEvoMontage "/Game/DigimonAnim/PlayerCharacter/Greymon/AnimMontage_GreymonEvo.AnimMontage_GreymonEvo")
  (bind _output_get (Variables|Default|SetSkillColldown 5.0))
  (Variables|Default|SetRemainTime _output_get)
  (Variables|Default|SetDie%20Montage "/Game/DigimonAnim/PlayerCharacter/Greymon/AM_Greymondie.AM_Greymondie")
  (Variables|Default|SetNextEvolutionName "/Game/DigimonAnim/PlayerCharacter/MetalGreymonBP/BP_MetalGreymon.BP_MetalGreymon_C")
  (Variables|Default|SetIn%20Socket%20Name "J_chin소켓")
  (Variables|Default|SetProjectileSpeed 1.5e+03)
  (Variables|Default|SetPortrait "/Game/DigimonAnim/PlayerCharacter/GreymonNew/Portrait_Type_D.Portrait_Type_D")
  (Variables|Default|SetLevelUpEmitter "/Game/InfinityBladeEffects/Effects/FX_Mobile/Fire/P_levelUp_Fire.P_levelUp_Fire")
  (Variables|Default|SetWidget%20Class "/Game/DigimonAnim/UI/SkillIcon/WBP_GreymonSkillIcon.WBP_GreymonSkillIcon_C")
  (Variables|Default|SetBase%20Damage 3.5e+02))

(event Collision|EventActorBeginOverlap
  (params (OtherActor :type Actor%20Object%20Reference)))

(event EventAttackCollisionStart
  (Collision|SetCollisionEnabled (Variables|Default|GetTail) "QueryAndPhysics"))

(event EventAttackCollisionEnd
  (Collision|SetCollisionEnabled (Variables|Default|GetTail) "NoCollision"))

(event EventTick
  (params (DeltaSeconds :type Float%20%28single-precision%29))
  (bind _playerslot (Variables|Default|GetPlayerSlot))
  (if (Variables|Default|GetActiveHeraldry)
    (bind _asbp_agumon_gamemode (Utilities|Casting|CastToBP_AgumonGamemode (Game|GetGameMode)))
    (if (>= (Variables|/Game/ThirdPerson/Blueprints/BP_AgumonGamemode.BP_AgumonGamemode_C|GetPlayer%20Level _asbp_agumon_gamemode) 5)
      (bind _array_index (Utilities|Array|ForEachLoopwithBreak _playerslot)
        (:LoopBody
          (if (== (.rowname (Utilities|Struct|BreakS_Slot (Utilities|Array|Get(acopy) _playerslot _array_index))) "CourageTag")
            (CallFunction|EquipHeraldry)))))))

(fn ConstructionScript
  (|CallParentFunction))