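; Base player character for a Digimon action game, handling movement, combat, item pickup, inventory and evolution.
; Montage attacks damage Monster-tagged actors, a cooldown-gated skill fires projectiles, and damage taken reduces HP stored in the game mode.
; Box-traced pickups fill a spawned backpack first, then player slots.
; Evolution, via video cutscene or heraldry, spawns and possesses the next character class, handing over backpack and slots before destroying the old pawn.
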(event Custom|ActorHitRelease
  ;[1 1 1] EndAttack
  (CallFunction|ActorCanHit (Variables|Default|GetIgnoreActor)))

(event Custom|UseSkill
  (bind _returnvalue (Game|GetPlayerController 0))
  (bind _returnvalue_2 (Pawn|GetControlledPawn _returnvalue))
  (bind _returnvalue_3 (Transformation|GetActorRotation _returnvalue_2))
  ;[1 1 1] SKill
  (if (<= (Variables|Default|GetSkillColldown) (Variables|Default|GetRemainTime))
    (bind _returnvalue_4 (Game|SpawnActorfromClass (Variables|Default|GetSpawnprojectile) (Math|Conversions|ToTransform(Vector) (Transformation|GetSocketLocation (Variables|Character|GetMesh) (Variables|Default|GetIn%20Socket%20Name))) "AlwaysSpawn" "MultiplyWithRoot" 0 0))
    (Utilities|IsValid _returnvalue_4
      (:Is%20Valid
        (bind _asbp_projectile (Utilities|Casting|CastToBP_Projectile _returnvalue_4))
        (Transformation|SetActorRotation _returnvalue_4 _returnvalue_3)
        (bind _output_get (Variables|Default|SetProjectile _asbp_projectile))
        (Variables|/Script/Engine.MovementComponent|SetVelocity (Variables|/Game/DigimonAnim/Skill/BP_Projectile.BP_Projectile_C|GetProjectileMovement _output_get) (* (Math|Vector|Normalize (Math|Vector|GetForwardVector _returnvalue_3)) (Variables|Default|GetProjectileSpeed)))
        (CallFunction|CoolDown)))))

(event Custom|AttackCollisionStart
  ;[1 1 1] CollisionEvent
)

(event Custom|AttackCollisionEnd
  ;[1 1 1] CollisionEvent
)

(event Custom|AttackEnd
  ;[1 1 1] EndAttack
  (if (not (Audio|Components|Audio|IsPlaying (Variables|Default|GetEvoScene)))
    (Variables|Default|SetIsAttack false)
    (CallFunction|ActorCanHit (Variables|Default|GetIgnoreActor))
    (Variables|Default|SetComboCount 0)
    (Variables|Default|SetCanNextAttack false)))

(event Custom|CoolDown
  (bind _skillcolldown (Variables|Default|GetSkillColldown))
  ;[1 1 1] CoolDown
  (bind _output_get (Variables|Default|SetRemainTime 0.0))
  (if (<= _output_get _skillcolldown) :!label _label
    (Utilities|FlowControl|Delay 0.1)
    (bind _output_get_2 (Variables|Default|SetRemainTime (+ _output_get 0.1)))
    (Variables|Default|SetSkillPercent (/ _output_get_2 _skillcolldown))
    (goto _label)))

(event Custom|Evo
  (Variables|Default|SetIsAttack true)
  (Variables|Actor|SetbCanBeDamaged false))

(event Custom|EvoEnd
  (Variables|Default|SetIsAttack false)
  (Variables|Actor|SetbCanBeDamaged true))

(event Custom|CutScene
  (bind _evoscene (Variables|Default|GetEvoScene))
  (bind _returnvalue (Media|MediaPlayer|GetDuration _evoscene))
  (CallFunction|Evo)
  (bind _returnvalue_2 (UserInterface|CreateWidget "/Game/DigimonAnim/UI/WBP_Evo.WBP_Evo_C"))
  (UserInterface|Viewport|AddtoViewport _returnvalue_2 0)
  (AddComponent|AddMediaSoundComponent false)
  (Media|MediaPlayer|OpenSource _evoscene (Variables|Default|GetMedia%20Source))
  (Utilities|FlowControl|Delay 0.2)
  (Utilities|FlowControl|Delay (+ (Math|Conversions|ToFloat(Integer) (.seconds _returnvalue)) (* (.milliseconds _returnvalue) 0.001)))
  (Media|MediaPlayer|Close _evoscene :!class /Script/MediaAssets.MediaPlayer)
  (Widget|RemovefromParent _returnvalue_2)
  (CallFunction|LevelUp)
  (CallFunction|NextEvolution)
  (bind _asbp_agumon_gamemode (Utilities|Casting|CastToBP_AgumonGamemode (Game|GetGameMode)))
  (Audio|Components|Audio|FadeIn (Variables|/Game/ThirdPerson/Blueprints/BP_AgumonGamemode.BP_AgumonGamemode_C|GetBG _asbp_agumon_gamemode) 1.0 1.0 0.0 "Linear" :!class /Script/Engine.AudioComponent))

(event Custom|RefreshWidget
  ;[1 1 1] Inventory
  (Utilities|FlowControl|Sequence
    (:then_0
      (Variables|/Script/Engine.PlayerController|SetbShowMouseCursor (Widget|GetOwningPlayer (Variables|Default|GetUI)) false)
      (Input|SetInputModeGameOnly (Widget|GetOwningPlayer (Variables|Default|GetUI)) false)
      (Widget|RemovefromParent (Variables|Default|GetUI)))
    (:then_1
      (bind _returnvalue (UserInterface|CreateWidget "/Game/DigimonAnim/UI/Inventoy/WBP_Inventory.WBP_Inventory_C"))
      (Variables|Default|SetUI _returnvalue)
      (UserInterface|Viewport|AddtoViewport (Variables|Default|GetUI) 0)
      (Variables|/Script/Engine.PlayerController|SetbShowMouseCursor (Widget|GetOwningPlayer (Variables|Default|GetUI)) true)
      (Input|SetInputModeGameandUI (Widget|GetOwningPlayer (Variables|Default|GetUI)) (Variables|Default|GetUI) "DoNotLock" true false))))

(event Input|EnhancedActionEvents|EnhancedInputActionIA_Move
  (params (ActionValue :type Vector%202D%20Structure) (ElapsedSeconds :type Float%20%28double-precision%29) (TriggeredSeconds :type Float%20%28double-precision%29) (InputAction :type Input%20Action%20Object%20Reference :default "/Game/ThirdPerson/Input/Actions/IA_Move.IA_Move"))
  (bind _returnvalue (Pawn|GetControlRotation :!class /Script/Engine.Pawn))
  ;[1 1 1] Move
  (if (not (Variables|Default|GetIsAttack))
    (Pawn|Input|AddMovementInput (Math|Vector|GetForwardVector (Math|Rotator|MakeRotator (.roll _returnvalue) 0.0 (.yaw _returnvalue))) (.y ActionValue) false)
    (Pawn|Input|AddMovementInput (Math|Vector|GetRightVector (Math|Rotator|MakeRotator 0.0 0.0 (.yaw (Pawn|GetControlRotation :!class /Script/Engine.Pawn)))) (.x ActionValue) false)))

(event Input|EnhancedActionEvents|EnhancedInputActionIA_Look
  (params (ActionValue :type Vector%202D%20Structure) (ElapsedSeconds :type Float%20%28double-precision%29) (TriggeredSeconds :type Float%20%28double-precision%29) (InputAction :type Input%20Action%20Object%20Reference :default "/Game/ThirdPerson/Input/Actions/IA_Look.IA_Look"))
  ;[1 1 1] Lood
  (Pawn|Input|AddControllerYawInput (.x ActionValue))
  (Pawn|Input|AddControllerPitchInput (.y ActionValue)))

(event Input|EnhancedActionEvents|EnhancedInputActionIA_Jump
  (params (ActionValue :type Boolean) (ElapsedSeconds :type Float%20%28double-precision%29) (TriggeredSeconds :type Float%20%28double-precision%29) (InputAction :type Input%20Action%20Object%20Reference :default "/Game/ThirdPerson/Input/Actions/IA_Jump.IA_Jump")))

(event Input|EnhancedActionEvents|EnhancedInputActionIA_Attack
  (params (ActionValue :type Boolean) (ElapsedSeconds :type Float%20%28double-precision%29) (TriggeredSeconds :type Float%20%28double-precision%29) (InputAction :type Input%20Action%20Object%20Reference :default "/Game/ThirdPerson/Input/Actions/IA_Attack.IA_Attack"))
  ;[1 1 1] Attack
  (:Started
    (if (Variables|Default|GetIsAttack)
      (Variables|Default|SetCanNextAttack true)
      (else
        (Animation|PlayAnimMontage (Variables|Default|GetAttack%20Montage) 1.0 "None")
        (Variables|Default|SetIsAttack true)))))

(event Input|EnhancedActionEvents|EnhancedInputActionIA_Skill
  (params (ActionValue :type Boolean) (ElapsedSeconds :type Float%20%28double-precision%29) (TriggeredSeconds :type Float%20%28double-precision%29) (InputAction :type Input%20Action%20Object%20Reference :default "/Game/ThirdPerson/Input/Actions/IA_Skill.IA_Skill"))
  ;[1 1 1] Skill
  (if (not (Variables|Default|GetIsAttack))
    (if (<= (Variables|Default|GetSkillColldown) (Variables|Default|GetRemainTime))
      (Animation|PlayAnimMontage (Variables|Default|GetSKillMontage) 1.0 "None")
      (Variables|Default|SetIsAttack true))))

(event EventBeginPlay
  ;[1 1 1] Init
  (bind _asbp_agumon_player (Utilities|Casting|CastToBP_AgumonPlayer (Pawn|GetController)))
  (Input|AddMappingContext (PlayerController|LocalPlayerSubsystems|GetEnhancedInputLocalPlayerSubsystem _asbp_agumon_player) "/Game/ThirdPerson/Input/IMC_Default.IMC_Default" 0 "(bIgnoreAllPressedKeysUntilRelease=True,bForceImmediately=False,bNotifyUserSettings=False)")
  (bind _asbp_agumon_gamemode (Utilities|Casting|CastToBP_AgumonGamemode (Game|GetGameMode)))
  (bind _output_get (Variables|Default|SetAs%20BP%20Gamemode _asbp_agumon_gamemode))
  (Default|Addwidget _output_get)
  (bind _returnvalue (Game|SpawnActorfromClass "/Game/DigimonAnim/UI/Inventoy/BP_BackPack.BP_BackPack_C" (Transformation|GetActorTransform (Game|Player|GetPlayerPawn 0)) "Undefined" "MultiplyWithRoot" 0 0))
  (Variables|Default|SetBackPack _returnvalue)
  (Audio|Components|Audio|Stop (Variables|Default|GetAudio)))

(event Game|Damage|EventAnyDamage
  (params (Damage :type Float%20%28single-precision%29) (DamageType :type Damage%20Type%20Object%20Reference) (InstigatedBy :type Controller%20Object%20Reference) (DamageCauser :type Actor%20Object%20Reference))
  (if (not (Variables|Default|GetIs%20Dying))
    (CallFunction|DamageTaken Damage)))

(event Input|KeyboardEvents|F
  (params (Key :type Key%20Structure :default "None"))
  (bind _mesh (Variables|Character|GetMesh))
  (bind _returnvalue (Transformation|GetWorldLocation _mesh))
  (bind _returnvalue_2 (Math|Vector|GetRightVector _mesh))
  ;[1 1 1] PickUp
  (:Pressed
    (bind (_outhit _returnvalue_3) (Collision|BoxTraceByChannel (+ _returnvalue (* _returnvalue_2 1)) (+ _returnvalue (* _returnvalue_2 500)) "200.000000,200.000000,200.000000" "0, 0, 0" "TraceTypeQuery3" false 0 "None"))
    (if _returnvalue_3
      (if (Actor|ActorHasTag (.HitActor (Collision|BreakHitResult _outhit)) "PickUp")
        (bind _asbp_pick_up_master (Utilities|Casting|CastToBP_PickUpMaster (.HitActor (Collision|BreakHitResult _outhit))))
        (bind _success (CallFunction|AddItem (Variables|/Game/DigimonAnim/UI/Inventoy/BP_PickUpMaster.BP_PickUpMaster_C|GetItem _asbp_pick_up_master) "Ground"))
        (if _success
          (Actor|DestroyActor _asbp_pick_up_master))))))

(event Input|KeyboardEvents|I
  (params (Key :type Key%20Structure :default "None"))
  ;[1 1 1] Inventory
  (:Pressed
    (Utilities|FlowControl|FlipFlop
      (:A
        (bind _returnvalue (UserInterface|CreateWidget "/Game/DigimonAnim/UI/Inventoy/WBP_Inventory.WBP_Inventory_C"))
        (Variables|Default|SetUI _returnvalue)
        (UserInterface|Viewport|AddtoViewport (Variables|Default|GetUI) 0)
        (Variables|/Script/Engine.PlayerController|SetbShowMouseCursor (Widget|GetOwningPlayer (Variables|Default|GetUI)) true)
        (Input|SetInputModeGameandUI (Widget|GetOwningPlayer (Variables|Default|GetUI)) (Variables|Default|GetUI) "DoNotLock" true false))
      (:B
        (Variables|/Script/Engine.PlayerController|SetbShowMouseCursor (Widget|GetOwningPlayer (Variables|Default|GetUI)) false)
        (Input|SetInputModeGameOnly (Widget|GetOwningPlayer (Variables|Default|GetUI)) false)
        (Widget|RemovefromParent (Variables|Default|GetUI))))))

(event Input|KeyboardEvents|Escape
  (params (Key :type Key%20Structure :default "None")))

(event Input|KeyboardEvents|Tab
  (params (Key :type Key%20Structure :default "None"))
  (bind _returnvalue (Game|GetPlayerController 0))
  (:Pressed
    (bind _returnvalue_2 (UserInterface|CreateWidget "/Game/DigimonAnim/UI/WBP_Pause.WBP_Pause_C"))
    (UserInterface|Viewport|AddtoViewport _returnvalue_2 0)
    (Variables|/Script/Engine.PlayerController|SetbShowMouseCursor _returnvalue true)
    (Input|SetInputModeGameandUI _returnvalue 0 "DoNotLock" true false)))

(event Input|KeyboardEvents|F11
  (params (Key :type Key%20Structure :default "None")))

(fn ConstructionScript)

(fn CheckHit
  (params (OtherActor :type Actor%20Object%20Reference))
  (bind _ignoreactor (Variables|Default|GetIgnoreActor))
  (if (not (== OtherActor self))
    (if (Actor|ActorHasTag OtherActor "Monster")
      (Utilities|Array|Insert _ignoreactor OtherActor (Utilities|Array|Length _ignoreactor))
      (if (Variables|/Script/Engine.Actor|GetbCanBeDamaged OtherActor)
        (Game|Damage|ApplyDamage OtherActor (Variables|Default|GetBase%20Damage) 0 self)
        (CameraShakes|StartCameraShake (Variables|/Script/Engine.PlayerController|GetPlayerCameraManager (Game|GetPlayerController 0)) "/Game/Camera/BP_CameraShake.BP_CameraShake_C" 1.0 "CameraLocal" "0, 0, 0")))))

(fn ActorCanHit
  (params (NewParam :type Array%20of%20Actor%20Object%20References))
  (if (Utilities|Array|IsNotEmpty NewParam)
    (for _array_element NewParam
      (Utilities|IsValid _array_element
        (:Is%20Valid
          (Variables|/Script/Engine.Actor|SetbCanBeDamaged _array_element true))))
    (Utilities|Array|Clear NewParam)))

(fn DamageTaken
  (params (Damage :type Float%20%28double-precision%29))
  (bind _returnvalue (Game|GetPlayerController 0))
  (Audio|Components|Audio|Play (Variables|Default|GetAudio) 0.0)
  (bind _asbp_agumon_gamemode (Utilities|Casting|CastToBP_AgumonGamemode (Game|GetGameMode)))
  (bind _output_get (Variables|/Game/ThirdPerson/Blueprints/BP_AgumonGamemode.BP_AgumonGamemode_C|SetPlayer%20HP _asbp_agumon_gamemode (- (Variables|/Game/ThirdPerson/Blueprints/BP_AgumonGamemode.BP_AgumonGamemode_C|GetPlayer%20HP _asbp_agumon_gamemode) Damage)))
  (if (<= _output_get 0.0)
    (Animation|PlayAnimMontage (Variables|Default|GetDie%20Montage) 1.0 "None")
    (Variables|Default|SetIs%20Dying true)
    (Input|DisableInput _returnvalue)
    (bind _returnvalue_2 (UserInterface|CreateWidget "/Game/DigimonAnim/UI/WBP_StageFailde.WBP_StageFailde_C" _returnvalue))
    (UserInterface|Viewport|AddtoViewport _returnvalue_2 0)
    (Variables|/Script/Engine.PlayerController|SetbShowMouseCursor _returnvalue true)
    (else
      (Animation|PlayAnimMontage (Variables|Default|GetHitMontage) 1.0 "None"))))

(fn NextEvolution
  (bind _returnvalue (Game|Player|GetPlayerPawn 0))
  (bind _returnvalue_2 (Transformation|GetActorTransform _returnvalue))
  (LocalVariables|SetLocalPlayerSlot (Variables|Default|GetPlayerSlot))
  (LocalVariables|SetLocalBackPack (Variables|Default|GetBackPack))
  (bind _returnvalue_3 (Game|SpawnActorfromClass (Variables|Default|GetNextEvolutionName) (Math|Transform|MakeTransform (.location _returnvalue_2) (.rotation _returnvalue_2) (.scale _returnvalue_2)) "AlwaysSpawn" "MultiplyWithRoot" 0 0))
  (bind _as폰 (Utilities|Casting|CastToPawn _returnvalue_3))
  (Pawn|Possess (Game|GetPlayerController 0) _as폰)
  (Actor|DestroyActor)
  (bind _asbp_base_character (Utilities|Casting|CastToBP_BaseCharacter _returnvalue_3))
  (Variables|BP_BaseCharacter_C|SetBackPack _asbp_base_character (LocalVariables|GetLocalBackPack))
  (Variables|BP_BaseCharacter_C|SetPlayerSlot _asbp_base_character (LocalVariables|GetLocalPlayerSlot))
  (Animation|PlayAnimMontage _asbp_base_character (Variables|BP_BaseCharacter_C|GetEvoMontage _asbp_base_character) 1.0 "None")
  (bind _asbp_agumon_gamemode (Utilities|Casting|CastToBP_AgumonGamemode (Game|GetGameMode)))
  (Default|Addwidget _asbp_agumon_gamemode))

(fn PrevEvolution
  (bind _returnvalue (Game|SpawnActorfromClass (Variables|Default|GetPrevEvolutionName) (Transformation|GetActorTransform (Game|Player|GetPlayerPawn 0)) "AlwaysSpawn" "MultiplyWithRoot" 0 0))
  (bind _as폰 (Utilities|Casting|CastToPawn _returnvalue))
  (Pawn|Possess (Game|GetPlayerController 0) _as폰)
  (Actor|DestroyActor))

(fn LevelUp
  (bind _returnvalue (Game|GetPlayerCharacter 0))
  (bind _returnvalue_2 (Transformation|GetActorLocation _returnvalue))
  (Effects|SpawnEmitteratLocation (Variables|Default|GetLevelUpEmitter) (Math|Vector|MakeVector (.x _returnvalue_2) (.y _returnvalue_2) (.z _returnvalue_2)) "0, 0, 0" "2.000000,2.000000,2.000000"))

(fn AddItem
  (params (Item :type S%20Slot%20Structure) (Source :type String))
  (bind _backpack (Variables|Default|GetBackPack))
  (LocalVariables|SetLocalItem Item)
  (switch string Source
    (:Ground
      (Utilities|IsValid _backpack
        (:Is%20Valid
          (bind _success (Default|AddItem _backpack (LocalVariables|GetLocalItem)))
          (if _success
            (return true)
            (else
              _)))
        (:Is%20Not%20Valid
          _))
      (bind (_success_2 _index) (CallFunction|FindStack (LocalVariables|GetLocalItem)))
      (if _success_2
        (bind _success_3 (CallFunction|AddItemtoPlayerSlot (LocalVariables|GetLocalItem) _index))
        (if _success_3
          (return _success_3)
          (else
            _)))
      (bind (_success_4 _index_2) (CallFunction|FindEmptySLot))
      (if _success_4
        (bind _success_5 (CallFunction|AddItemtoPlayerSlot (LocalVariables|GetLocalItem) _index_2))
        (return _success_5)
        (else
          (return false))))))

(fn FindStack
  (params (Item :type S%20Slot%20Structure))
  (bind (_array_element _array_index) (Utilities|Array|ForEachLoopwithBreak (Variables|Default|GetPlayerSlot) :!label _label)
    (:LoopBody
      (if (== (.RowName (Utilities|Struct|BreakDataTableRowHandle (Utilities|Struct|BreakS_Slot _array_element))) (.RowName (Utilities|Struct|BreakDataTableRowHandle (Utilities|Struct|BreakS_Slot Item))))
        (LocalVariables|SetLocalFound true)
        (LocalVariables|SetLoaclIndex _array_index)
        (goto _label Break)))
    (:Completed
      (return (LocalVariables|GetLocalFound) (LocalVariables|GetLoaclIndex)))))

(fn FindEmptySLot
  (bind (_array_element _array_index) (Utilities|Array|ForEachLoopwithBreak (Variables|Default|GetPlayerSlot) :!label _label)
    (:LoopBody
      (if (== (.RowName (Utilities|Struct|BreakDataTableRowHandle (Utilities|Struct|BreakS_Slot _array_element))) "Empty")
        (LocalVariables|SetLocalFound true)
        (LocalVariables|SetLocalIndex _array_index)
        (goto _label Break)))
    (:Completed
      (return (LocalVariables|GetLocalFound) (LocalVariables|GetLocalIndex)))))

(fn Removeitem
  (params (Item :type S%20Slot%20Structure))
  (bind (_success _index) (CallFunction|FindStack Item))
  (if _success
    (Utilities|Array|SetArrayElem (Variables|Default|GetPlayerSlot) _index (Utilities|Struct|MakeS_Slot (Utilities|Struct|MakeDataTableRowHandle "/Game/DigimonAnim/UI/Inventoy/SelectItemp.SelectItemp" "Empty")))
    (return true)
    (else
      (return false))))

(fn AddItemtoPlayerSlot
  (params (Itme :type S%20Slot%20Structure) (Index :type Integer))
  (LocalVariables|SetLoaclItem Itme)
  (LocalVariables|SetLocalIndex Index)
  (if (== (.RowName (Utilities|Struct|BreakDataTableRowHandle (.itme (Utilities|Array|Get(acopy) (Variables|Default|GetPlayerSlot) (LocalVariables|GetLocalIndex))))) "Empty")
    (Utilities|Array|SetArrayElem (Variables|Default|GetPlayerSlot) (LocalVariables|GetLocalIndex) (LocalVariables|GetLoaclItem))
    (return true)
    (else
      (bind _returnvalue (Utilities|GetDataTableRow (.DataTable (Utilities|Struct|BreakDataTableRowHandle (.itme (LocalVariables|GetLoaclItem)))) (.RowName (Utilities|Struct|BreakDataTableRowHandle (.itme (LocalVariables|GetLoaclItem)))))
        (:then
          (if (and (.CanStack (Utilities|Struct|BreakS_Inventory _returnvalue)) (== (.RowName (Utilities|Struct|BreakDataTableRowHandle (.itme (Utilities|Array|Get(acopy) (Variables|Default|GetPlayerSlot) (LocalVariables|GetLocalIndex))))) (.RowName (Utilities|Struct|BreakDataTableRowHandle (.itme (LocalVariables|GetLoaclItem))))))
            (Utilities|Array|SetArrayElem (Variables|Default|GetPlayerSlot) (LocalVariables|GetLocalIndex) (Utilities|Struct|MakeS_Slot (.itme (LocalVariables|GetLoaclItem))))
            (return true)
            (else
              (return false))))
        (:RowNotFound
          (return false))))))

(fn EquipHeraldry
  (bind _returnvalue (Game|GetPlayerController 0))
  (bind _ui (Variables|Default|GetUI))
  (Variables|Default|SetActiveHeraldry false)
  (Utilities|IsValid _ui
    (:Is%20Valid
      (Variables|/Script/Engine.PlayerController|SetbShowMouseCursor _returnvalue false)
      (Input|SetInputModeGameOnly _returnvalue false)
      (Widget|RemovefromParent _ui))
    (:Is%20Not%20Valid
      _))
  (CallFunction|Evo)
  (CallFunction|LevelUp)
  (CallFunction|NextEvolution)
  (bind _asbp_agumon_gamemode (Utilities|Casting|CastToBP_AgumonGamemode (Game|GetGameMode)))
  (bind _asbp_base_character (Utilities|Casting|CastToBP_BaseCharacter (Game|GetPlayerCharacter 0)))
  (Variables|/Game/ThirdPerson/Blueprints/BP_AgumonGamemode.BP_AgumonGamemode_C|SetAs%20BP%20Base%20Character _asbp_agumon_gamemode _asbp_base_character)
  (return true))