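; BP_MetalGreymon is the player's MetalGreymon character, one evolution stage between Greymon and WarGreymon.
; BeginPlay fills the parent class's montages, stats, UI and evolution data.
; A left-hand collider, toggled during attacks, checks hits, while the cooldown-gated skill fires missiles from both hatch sockets along the pawn's facing.
; With heraldry active, Tick checks for player level five and an inventory CourageTag before calling EquipHeraldry.
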(event OnComponentBeginOverlap(LeftHand)
  (params (OverlappedComponent :type Primitive%20Component%20Object%20Reference) (OtherActor :type Actor%20Object%20Reference) (OtherComp :type Primitive%20Component%20Object%20Reference) (OtherBodyIndex :type Integer) (bFromSweep :type Boolean) (SweepResult :type Hit%20Result%20Structure%20%28by%20ref%29))
  (CallFunction|CheckHit OtherActor))

(event Custom|AttackCollsionStart
  (Collision|SetCollisionEnabled (Variables|Default|GetLeftHand) "QueryAndPhysics"))

(event Custom|AttackCollsionEnd
  (Collision|SetCollisionEnabled (Variables|Default|GetLeftHand) "NoCollision"))

(event EventBeginPlay
  (|CallParentFunction)
  (Variables|Default|SetAttack%20Montage "/Game/DigimonAnim/PlayerCharacter/MetalGreymon/AnimMontage_MetalGreymonAttack.AnimMontage_MetalGreymonAttack")
  (Variables|Default|SetSKillMontage "/Game/DigimonAnim/PlayerCharacter/MetalGreymon/AnimMontage_MetalGreymonSkill.AnimMontage_MetalGreymonSkill")
  (Variables|Default|SetSpawnprojectile "/Game/DigimonAnim/Skill/BP_Missile.BP_Missile_C")
  (Variables|Default|SetPrevEvolutionName "/Game/DigimonAnim/PlayerCharacter/GreymonNew/BP_Greymon.BP_Greymon_C")
  (bind _output_get (Variables|Default|SetSkillColldown 5.0))
  (Variables|Default|SetRemainTime _output_get)
  (Variables|Default|SetEvoMontage "/Game/DigimonAnim/PlayerCharacter/MetalGreymon/AnimMontage_MetalGreyEvo.AnimMontage_MetalGreyEvo")
  (Variables|Default|SetDie%20Montage "/Game/DigimonAnim/PlayerCharacter/MetalGreymon/AM_MetalGreyDie.AM_MetalGreyDie")
  (Variables|Default|SetNextEvolutionName "/Game/DigimonAnim/PlayerCharacter/WarGreymonBP/BP_WarGreymonBP.BP_WarGreymonBP_C")
  (Variables|Default|SetIn%20Socket%20Name "L_Hatch")
  (Variables|Default|SetProjectileSpeed 2.5e+03)
  (Variables|Default|SetPortrait "/Game/DigimonAnim/PlayerCharacter/MetalGreymonBP/Portrait_Type_D.Portrait_Type_D")
  (Variables|Default|SetLevelUpEmitter "/Game/InfinityBladeEffects/Effects/FX_Mobile/Fire/P_levelUp_Fire.P_levelUp_Fire")
  (Variables|Default|SetWidget%20Class "/Game/DigimonAnim/UI/SkillIcon/WBP_MetalGrey.WBP_MetalGrey_C")
  (Variables|Default|SetBase%20Damage 5e+02)
  (Variables|Default|SetEvoScene "/Game/DigimonAnim/NewMediaPlayer.NewMediaPlayer")
  (Variables|Default|SetMedia%20Source "/Game/Movies/wargrey2.wargrey2"))

(event EventUseSkill
  ;[1 1 1] SKill
  (if (<= (Variables|Default|GetSkillColldown) (Variables|Default|GetRemainTime))
    (Utilities|FlowControl|Sequence
      (:then_0
        (CallFunction|SpawnMissile "R_HatchSocket")
        (CallFunction|CoolDown))
      (:then_1
        (CallFunction|SpawnMissile "L_HatchSocket")))))

(event EventTick
  (params (DeltaSeconds :type Float%20%28single-precision%29))
  (bind _playerslot (Variables|Default|GetPlayerSlot))
  (if (Variables|Default|GetActiveHeraldry)
    (bind _asbp_agumon_gamemode (Utilities|Casting|CastToBP_AgumonGamemode (Game|GetGameMode)))
    (if (>= (Variables|/Game/ThirdPerson/Blueprints/BP_AgumonGamemode.BP_AgumonGamemode_C|GetPlayer%20Level _asbp_agumon_gamemode) 5)
      (bind _array_index (Utilities|Array|ForEachLoopwithBreak _playerslot)
        (:LoopBody
          (if (== (.rowname (Utilities|Struct|BreakS_Slot (Utilities|Array|Get(acopy) _playerslot _array_index))) "CourageTag")
            (CallFunction|EquipHeraldry)))))))

(fn ConstructionScript
  (|CallParentFunction))

(fn SpawnMissile
  (params (SocketName :type Name))
  (bind _returnvalue (Game|GetPlayerController 0))
  (bind _returnvalue_2 (Pawn|GetControlledPawn _returnvalue))
  (bind _returnvalue_3 (Transformation|GetActorRotation _returnvalue_2))
  (bind _returnvalue_4 (Game|SpawnActorfromClass "/Game/DigimonAnim/Skill/BP_Missile.BP_Missile_C" (Math|Conversions|ToTransform(Vector) (Transformation|GetSocketLocation (Variables|Character|GetMesh) SocketName)) "AlwaysSpawn" "MultiplyWithRoot" 0 0))
  (bind _asbp_projectile (Utilities|Casting|CastToBP_Projectile _returnvalue_4))
  (Transformation|SetActorRotation _returnvalue_4 _returnvalue_3)
  (bind _output_get (Variables|Default|SetProjectile _asbp_projectile))
  (Variables|/Script/Engine.MovementComponent|SetVelocity (Variables|/Game/DigimonAnim/Skill/BP_Projectile.BP_Projectile_C|GetProjectileMovement _output_get) (* (Math|Vector|Normalize (Math|Vector|GetForwardVector _returnvalue_3)) (Variables|Default|GetProjectileSpeed))))