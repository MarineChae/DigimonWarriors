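; BP_Agumon is the Agumon player character, a child Blueprint that configures its parent's shared Digimon logic.
; BeginPlay calls the parent, then fills in montages, fireball projectile, damage, UI assets and Greymon as the next evolution, with no previous form.
; AttackCollisionStart and AttackCollisionEnd toggle collision on both hand components, limiting melee hits to attack windows.
; Overlaps on either hand pass the other actor to CheckHit.
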(event OnComponentBeginOverlap(LeftHand)
  (params (OverlappedComponent :type Primitive%20Component%20Object%20Reference) (OtherActor :type Actor%20Object%20Reference) (OtherComp :type Primitive%20Component%20Object%20Reference) (OtherBodyIndex :type Integer) (bFromSweep :type Boolean) (SweepResult :type Hit%20Result%20Structure%20%28by%20ref%29))
  (CallFunction|CheckHit OtherActor))

(event OnComponentBeginOverlap(RightHand)
  (params (OverlappedComponent :type Primitive%20Component%20Object%20Reference) (OtherActor :type Actor%20Object%20Reference) (OtherComp :type Primitive%20Component%20Object%20Reference) (OtherBodyIndex :type Integer) (bFromSweep :type Boolean) (SweepResult :type Hit%20Result%20Structure%20%28by%20ref%29))
  (CallFunction|CheckHit OtherActor))

(event EventBeginPlay
  (|CallParentFunction)
  (Variables|Default|SetAttack%20Montage "/Game/DigimonAnim/PlayerCharacter/Agumon2/AnimMontage_Attack.AnimMontage_Attack")
  (Variables|Default|SetSKillMontage "/Game/DigimonAnim/PlayerCharacter/Agumon2/AnimMontage_Skill.AnimMontage_Skill")
  (Variables|Default|SetSpawnprojectile "/Game/DigimonAnim/Skill/BP_FireBall.BP_FireBall_C")
  (Variables|Default|SetPrevEvolutionName 0)
  (Variables|Default|SetWidget%20Class "/Game/DigimonAnim/UI/SkillIcon/WBP_SkillIcon.WBP_SkillIcon_C")
  (Variables|Default|SetEvoMontage "/Game/DigimonAnim/PlayerCharacter/Greymon/AnimMontage_GreymonEvo.AnimMontage_GreymonEvo")
  (Variables|Default|SetDie%20Montage "/Game/DigimonAnim/PlayerCharacter/Agumon2/AnimMontage_Agumondie.AnimMontage_Agumondie")
  (Variables|Default|SetNextEvolutionName "/Game/DigimonAnim/PlayerCharacter/GreymonNew/BP_Greymon.BP_Greymon_C")
  (Variables|Default|SetIn%20Socket%20Name "J_joeSocket")
  (Variables|Default|SetProjectileSpeed 1.5e+03)
  (Variables|Default|SetPortrait "/Game/Portrait/Portrait_Type_D.Portrait_Type_D")
  (Variables|Default|SetLevelUpEmitter "/Game/InfinityBladeEffects/Effects/FX_Mobile/Fire/P_levelUp_Fire.P_levelUp_Fire")
  (Variables|Default|SetWidget%20Class "/Game/DigimonAnim/UI/SkillIcon/WBP_SkillIcon.WBP_SkillIcon_C")
  (Variables|Default|SetBase%20Damage 1e+02))

(event Collision|EventActorBeginOverlap
  (params (OtherActor :type Actor%20Object%20Reference)))

(event EventTick
  (params (DeltaSeconds :type Float%20%28single-precision%29)))

(event EventAttackCollisionStart
  (Collision|SetCollisionEnabled (Variables|Default|GetLeftHand) "QueryAndPhysics")
  (Collision|SetCollisionEnabled (Variables|Default|GetRightHand) "QueryAndPhysics"))

(event EventAttackCollisionEnd
  (Collision|SetCollisionEnabled (Variables|Default|GetLeftHand) "NoCollision")
  (Collision|SetCollisionEnabled (Variables|Default|GetRightHand) "NoCollision"))

(fn ConstructionScript
  (|CallParentFunction))