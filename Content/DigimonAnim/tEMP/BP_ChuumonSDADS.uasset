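; Chuumon enemy character that plays an attack montage and throws cheese projectiles along its facing direction.
; Tick caches distance and direction to the player and keeps a separately spawned HP bar actor positioned and turned along that direction.
; Pick, throw and attack-end events drive the hand cheese mesh, projectile spawn and attack flag.
; Damage triggers hit-and-turn or death; FireDamage applies fixed damage without a hit reaction, and Endfire clears a timer.
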(event Custom|Save%20Dis&Dir
  (bind _returnvalue (Game|GetPlayerController 0))
  (bind _returnvalue_2 (Transformation|GetActorLocation))
  (bind _returnvalue_3 (Pawn|GetControlledPawn _returnvalue))
  (bind _returnvalue_4 (Transformation|GetActorLocation _returnvalue_3))
  (bind _returnvalue_5 (- _returnvalue_4 _returnvalue_2))
  (bind (_x _y _z) (Math|Vector|BreakVector _returnvalue_5))
  (bind _returnvalue_6 (Math|Vector|MakeVector _x _y _z))
  ;[1 1 1] Dis&Dir to Player
  (Variables|Default|SetDistance%20To%20Player (Math|Vector|VectorLength _returnvalue_6))
  (Variables|Default|SetDirection%20To%20Player (Math|Vector|Normalize _returnvalue_6)))

(event Custom|Attack
  ;[1 1 1] Attack
  (Animation|PlayAnimMontage "/Game/DigimonAnim/Enemy/Chuumon/AnimMontage_ChuumonAttack.AnimMontage_ChuumonAttack" 1.0 "None")
  (Variables|Default|SetIsAttack true))

(event Custom|PickCheese
  ;[1 1 1] Projectile
  (Development|SetHiddeninGame (Variables|Default|GetStaticMesh) false false))

(event Custom|ThrowCheese
  ;[1 1 1] Projectile
  (Development|SetHiddeninGame (Variables|Default|GetStaticMesh) true false)
  (bind _returnvalue (Game|SpawnActorfromClass "/Game/DigimonAnim/Skill/BP_Cheese.BP_Cheese_C" (Math|Conversions|ToTransform(Vector) (Transformation|GetSocketLocation (Variables|Default|GetStaticMesh) "J_hand_R소켓")) "Undefined" "MultiplyWithRoot" self 0))
  (Utilities|IsValid _returnvalue
    (:Is%20Valid
      (bind _output_get (Variables|Default|SetProjectile _returnvalue))
      (Variables|/Script/Engine.MovementComponent|SetVelocity (Variables|/Game/DigimonAnim/Skill/BP_Projectile.BP_Projectile_C|GetProjectileMovement _output_get) (* (Math|Vector|Normalize (Math|Vector|GetForwardVector (Transformation|GetActorRotation))) 1.5e+03)))))

(event Custom|AttackEnd
  ;[1 1 1] Attack
  (Variables|Default|SetIsAttack false))

(event EventTick
  (params (DeltaSeconds :type Float%20%28single-precision%29))
  (bind _hpwidget (Variables|Default|GetHPWidget))
  (CallFunction|SaveDis&Dir)
  (Utilities|IsValid _hpwidget
    (:Is%20Valid
      (Default|UpdateLocation _hpwidget (Transformation|GetWorldLocation (Variables|Default|GetHpBar)))
      (Default|UpdateRotate _hpwidget (Math|Conversions|RotationFromXVector (Variables|Default|GetDirection%20to%20Player))))))

(event Game|Damage|EventAnyDamage
  (params (Damage :type Float%20%28single-precision%29) (DamageType :type Damage%20Type%20Object%20Reference) (InstigatedBy :type Controller%20Object%20Reference) (DamageCauser :type Actor%20Object%20Reference))
  ;[1 1 1] Damage Taken
  (if (not (Variables|Default|GetIs%20Dying))
    (bind _output_get (Variables|Default|SetHP (- (Variables|Default|GetHP) Damage)))
    (Default|UpdateHpBar (Variables|Default|GetHPWidget) _output_get (Variables|Default|GetMax%20HP))
    (if (<= _output_get 0.0)
      (bind _output_get_2 (Variables|Default|SetAnim%20Montage "/Game/DigimonAnim/Enemy/Chuumon/AnimMontage_ChumonDie.AnimMontage_ChumonDie"))
      (Animation|PlayAnimMontage _output_get_2 1.0 "None")
      (Variables|Default|SetIs%20Dying true)
      (Collision|SetCollisionEnabled (Variables|Collision|GetCapsuleComponent) "NoCollision")
      (Collision|SetCollisionEnabled (Variables|Character|GetMesh) "NoCollision")
      (Actor|DestroyActor (Variables|Default|GetHPWidget))
      (else
        (Variables|Default|SetAnim%20Montage 0)
        (bind _returnvalue (Animation|PlayAnimMontage "/Game/DigimonAnim/Enemy/Chuumon/AnimMontage_ChumonHit.AnimMontage_ChumonHit" 1.0 "None"))
        (Transformation|SetActorRotation (Math|Conversions|RotationFromXVector (Variables|Default|GetDirection%20to%20Player)))
        (Development|SetHiddeninGame (Variables|Default|GetStaticMesh) true false)
        (Utilities|FlowControl|Delay _returnvalue)
        (Variables|Default|SetIsAttack false)))))

(event EventBeginPlay
  ;[1 1 1] Init
  (Development|SetHiddeninGame (Variables|Default|GetStaticMesh) true false)
  (bind _returnvalue (Game|SpawnActorfromClass "/Game/DigimonAnim/UI/BP_HPWidget.BP_HPWidget_C" (Math|Transform|MakeTransform (Transformation|GetWorldLocation (Variables|Default|GetHpBar))) "Undefined" "MultiplyWithRoot" 0 0))
  (Variables|Default|SetHPWidget _returnvalue))

(fn ConstructionScript)

(fn UpdateWalkSpeed
  (params (NewWalkSpeed :type Float%20%28double-precision%29))
  (Variables|/Script/Engine.CharacterMovementComponent|SetMaxWalkSpeed (Variables|Character|GetCharacterMovement) NewWalkSpeed))

(fn FireDamage
  (bind _output_get (Variables|Default|SetHP (- (Variables|Default|GetHP) 2e+01)))
  (Default|UpdateHpBar (Variables|Default|GetHPWidget) _output_get (Variables|Default|GetMax%20HP))
  (if (<= _output_get 0.0)
    (bind _output_get_2 (Variables|Default|SetAnim%20Montage "/Game/DigimonAnim/Enemy/Chuumon/AnimMontage_ChumonDie.AnimMontage_ChumonDie"))
    (Animation|PlayAnimMontage _output_get_2 1.0 "None")
    (Variables|Default|SetIs%20Dying true)
    (Collision|SetCollisionEnabled (Variables|Collision|GetCapsuleComponent) "NoCollision")
    (Collision|SetCollisionEnabled (Variables|Character|GetMesh) "NoCollision")
    (Actor|DestroyActor (Variables|Default|GetHPWidget))))

(fn Endfire
  (Utilities|Time|ClearandInvalidateTimerbyHandle (Variables|Default|GetTimer)))