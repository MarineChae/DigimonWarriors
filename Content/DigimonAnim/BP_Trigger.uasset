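; Boss encounter trigger that starts the VenomVamdemon intro cutscene the first time a Player-tagged actor overlaps it.
; It crossfades the game mode's background music to the boss track, hides the boss, plays a level sequence and turns the sky light bright magenta.
; A timer derived from the sequence's frame count at an assumed 30 fps then unhides the boss and destroys the trigger.
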(event Custom|ViewEnemy
  (bind _returnvalue (Actor|GetActorOfClass "/Game/DigimonAnim/Enemy/VenomVamdemonBP/BP_VenomVamdemon.BP_VenomVamdemon_C"))
  (Rendering|SetActorHiddenInGame _returnvalue false)
  (Actor|DestroyActor))

(event EventBeginPlay)

(event Collision|EventActorBeginOverlap
  (params (OtherActor :type Actor%20Object%20Reference))
  (if (and (Actor|ActorHasTag OtherActor "Player") (not (Variables|Default|GetIsPlay)))
    (CallFunction|ChageAudio)
    (bind _returnvalue (Actor|GetActorOfClass "/Game/DigimonAnim/Enemy/VenomVamdemonBP/BP_VenomVamdemon.BP_VenomVamdemon_C"))
    (Rendering|SetActorHiddenInGame _returnvalue true)
    (bind _returnvalue_2 (Sequencer|Player|CreateLevelSequencePlayer "/Game/Movies/NewLevelSequence.NewLevelSequence"))
    (Variables|Default|SetScenePlay _returnvalue_2)
    (Sequencer|Player|Play _returnvalue_2 :!class /Script/MovieScene.MovieSceneSequencePlayer)
    (Utilities|Time|SetTimerbyEvent (delegate Custom|ViewEnemy) (/ (Class|TimeManagementBlueprintLibrary|ToInteger(FrameNumber) (.frame (Media|MediaPlayer|GetDuration _returnvalue_2))) 30))
    (bind _returnvalue_3 (Actor|GetActorOfClass "/Game/DigimonAnim/BP_SkyLight.BP_SkyLight_C"))
    (Rendering|Components|Light|SetLightColor (Variables|/Script/Engine.SkyLight|GetLightComponent _returnvalue_3) "(R=1.000000,G=0.000000,B=1.000000,A=1.000000)")
    (Rendering|Components|Light|SetIntensity (Variables|/Script/Engine.SkyLight|GetLightComponent _returnvalue_3) 2e+02)
    (Variables|Default|SetIsPlay true)))

(fn ConstructionScript)

(fn ChageAudio
  (bind _asbp_agumon_gamemode (Utilities|Casting|CastToBP_AgumonGamemode (Game|GetGameMode)))
  (Audio|Components|Audio|FadeOut (Variables|/Game/ThirdPerson/Blueprints/BP_AgumonGamemode.BP_AgumonGamemode_C|GetBG _asbp_agumon_gamemode) 1.0 0.0 "Linear" :!class /Script/Engine.AudioComponent)
  (Audio|Components|Audio|FadeIn (Variables|/Game/ThirdPerson/Blueprints/BP_AgumonGamemode.BP_AgumonGamemode_C|GetBossSound _asbp_agumon_gamemode) 1.0 1.0 0.0 "Linear" :!class /Script/Engine.AudioComponent))