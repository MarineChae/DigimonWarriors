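; BP_BlueFire is a short-lived blue fire skill actor that damages actors overlapping it, excluding the player character.
; Delays on Tick repeatedly toggle the Capsule's collision off and on about every 0.2 seconds, refreshing overlaps, and destroy the actor after about one second.
; Each begin-overlap calls FireDamage, which applies fixed damage credited to the first player's controller.
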(event EventBeginPlay)

(event Collision|EventActorBeginOverlap
  (params (OtherActor :type Actor%20Object%20Reference))
  (CallFunction|FireDamage OtherActor))

(event EventTick
  (params (DeltaSeconds :type Float%20%28single-precision%29))
  (bind _capsule (Variables|Default|GetCapsule))
  (Utilities|FlowControl|Sequence
    (:then_0
      (Utilities|FlowControl|Delay 0.2)
      (Collision|SetCollisionEnabled _capsule "NoCollision")
      (Collision|SetCollisionEnabled _capsule "QueryAndPhysics"))
    (:then_1
      (Utilities|FlowControl|Delay 1.0)
      (Utilities|IsValid self
        (:Is%20Valid
          (Actor|DestroyActor))))))

(fn ConstructionScript)

(fn FireDamage
  (params (액터 :type Actor%20Object%20Reference))
  (if (!= 액터 (Game|GetPlayerCharacter 0))
    (Game|Damage|ApplyDamage 액터 2e+02 (Game|GetPlayerController 0) self)))