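; BP_EtemonSkill is a skill actor for Etemon that explodes when it overlaps an actor tagged Player.
; On contact it applies full radial damage, ignoring the BP_Etemon found in the level, spawns explosion particles and sound, then destroys itself.
; The Ete component plays from BeginPlay until EndPlay.
; Tick runs a short Delay before DestroyActor, acting as a lifetime limit.
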(event EventBeginPlay
  (|CallParentFunction)
  (Audio|Components|Audio|Play (Variables|Default|Getete) 0.0))

(event Collision|EventActorBeginOverlap
  (params (OtherActor :type Actor%20Object%20Reference))
  (bind _returnvalue (Transformation|GetActorLocation))
  (bind _returnvalue_2 (Actor|GetActorOfClass "/Game/DigimonAnim/Enemy/EtemonBP/BP_Etemon.BP_Etemon_C"))
  (if (Actor|ActorHasTag OtherActor "Player")
    (Game|Damage|ApplyRadialDamage (Variables|Default|GetDamage) _returnvalue 7e+02 0 (Utilities|Array|MakeArray _returnvalue_2) self (AI|GetAIController 0) true "ECC_WorldDynamic")
    (Effects|SpawnEmitteratLocation "/Game/MilitaryWeapDark/FX/P_RocketLauncher_Explosion_01.P_RocketLauncher_Explosion_01" _returnvalue "0, 0, 0" "5.000000,5.000000,5.000000")
    (Audio|SpawnSoundatLocation "/Game/Sound/Explosion02.Explosion02" _returnvalue "0, 0, 0" 1.0 1.0 0.0 0 0)
    (Actor|DestroyActor)))

(event EventEndPlay
  (params (EndPlayReason :type EEndPlayReason%20Enum :default "Destroyed"))
  (Audio|Components|Audio|Stop (Variables|Default|Getete)))

(event EventTick
  (params (DeltaSeconds :type Float%20%28single-precision%29))
  (Utilities|FlowControl|Delay 3.0)
  (Actor|DestroyActor))

(fn ConstructionScript
  (|CallParentFunction))