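; BP_Cheese is a Digimon skill hazard actor that damages whatever tagged Player or Plane overlaps it.
; On overlap it applies BaseDamage, passing an AI controller as instigator and its root component's owner as causer.
; It then spawns a scaled-down rocket explosion effect with a quieter explosion sound and destroys itself.
; The graphs contain no movement or spawning logic for the actor itself.
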(event EventBeginPlay
  (|CallParentFunction) ; 지금 이 노드는 비활성 상태입니다. \n핀을 끌어서 다른 노드를 연결하면 활성화됩니다.
)

(event Collision|EventActorBeginOverlap
  (params (OtherActor :type Actor%20Object%20Reference))
  (bind _returnvalue (Transformation|GetActorLocation))
  (if (or (Actor|ActorHasTag OtherActor "Player") (Actor|ActorHasTag OtherActor "Plane"))
    (Game|Damage|ApplyDamage OtherActor (Variables|Default|GetBase%20Damage) (AI|GetAIController 0) (Components|GetOwner (Variables|Default|GetDefaultSceneRoot)))
    (Effects|SpawnEmitteratLocation "/Game/MilitaryWeapDark/FX/P_RocketLauncher_Explosion_01.P_RocketLauncher_Explosion_01" _returnvalue "0, 0, 0" "0.200000,0.200000,0.200000")
    (Audio|SpawnSoundatLocation "/Game/Sound/Explosion01.Explosion01" _returnvalue "0, 0, 0" 0.2 1.0 0.0 0 0)
    (Actor|DestroyActor)))

(event EventTick
  (params (DeltaSeconds :type Float%20%28single-precision%29))
  (|CallParentFunction DeltaSeconds) ; 지금 이 노드는 비활성 상태입니다. \n핀을 끌어서 다른 노드를 연결하면 활성화됩니다.
)

(fn ConstructionScript
  (|CallParentFunction))