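; BP_MegaFire is a Digimon skill actor that explodes when it overlaps any actor other than the player character.
; On overlap it applies full radial damage from its Damage variable around itself, sparing the player's controlled pawn and crediting the player's controller.
; It then spawns a scaled-up rocket explosion emitter and sound and destroys itself.
; The Sphere hit event is empty, and BeginPlay and Tick are disabled.
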(event OnComponentHit(Sphere)
  (params (HitComponent :type Primitive%20Component%20Object%20Reference) (OtherActor :type Actor%20Object%20Reference) (OtherComp :type Primitive%20Component%20Object%20Reference) (NormalImpulse :type Vector :default "0, 0, 0") (Hit :type Hit%20Result%20Structure%20%28by%20ref%29)))

(event EventBeginPlay
  (|CallParentFunction) ; 지금 이 노드는 비활성 상태입니다. \n핀을 끌어서 다른 노드를 연결하면 활성화됩니다.
)

(event Collision|EventActorBeginOverlap
  (params (OtherActor :type Actor%20Object%20Reference))
  (bind _returnvalue (Transformation|GetActorLocation))
  (bind _returnvalue_2 (Game|GetPlayerController 0))
  (if (!= OtherActor (Game|GetPlayerCharacter 0))
    (Game|Damage|ApplyRadialDamage (Variables|Default|GetDamage) _returnvalue 1e+03 0 (Utilities|Array|MakeArray (Pawn|GetControlledPawn _returnvalue_2)) self _returnvalue_2 true "ECC_WorldDynamic")
    (Effects|SpawnEmitteratLocation "/Game/MilitaryWeapDark/FX/P_RocketLauncher_Explosion_01.P_RocketLauncher_Explosion_01" _returnvalue "0, 0, 0" "2.000000,2.000000,2.000000")
    (Audio|SpawnSoundatLocation "/Game/Sound/Explosion02.Explosion02" _returnvalue "0, 0, 0" 1.0 1.0 0.0 0 0)
    (Actor|DestroyActor)))

(event EventTick
  (params (DeltaSeconds :type Float%20%28single-precision%29))
  (|CallParentFunction DeltaSeconds) ; 지금 이 노드는 비활성 상태입니다. \n핀을 끌어서 다른 노드를 연결하면 활성화됩니다.
)

(fn ConstructionScript
  (|CallParentFunction))