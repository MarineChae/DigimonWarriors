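; BP_IceSpere is an ice skill actor that damages the Player or Plane on contact.
; On overlap with an actor tagged Player or Plane, it applies BaseDamage with an AI controller as instigator, spawns an ice-break particle and explosion sound, then destroys itself.
; Other overlaps are ignored, and the graph has no movement logic or active BeginPlay and Tick behavior.
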(event EventBeginPlay
  (|CallParentFunction) ; 지금 이 노드는 비활성 상태입니다. \n핀을 끌어서 다른 노드를 연결하면 활성화됩니다.
)

(event Collision|EventActorBeginOverlap
  (params (OtherActor :type Actor%20Object%20Reference))
  (bind _returnvalue (Transformation|GetActorLocation))
  (if (or (Actor|ActorHasTag OtherActor "Player") (Actor|ActorHasTag OtherActor "Plane"))
    (Game|Damage|ApplyDamage OtherActor (Variables|Default|GetBase%20Damage) (AI|GetAIController 0) (Components|GetOwner (Variables|Default|GetDefaultSceneRoot)))
    (Effects|SpawnEmitteratLocation "/Game/InfinityBladeEffects/Effects/FX_Mobile/ICE/combat/P_Break_IceWall.P_Break_IceWall" _returnvalue (Transformation|GetActorRotation))
    (Audio|SpawnSoundatLocation "/Game/Sound/Explosion02.Explosion02" _returnvalue "0, 0, 0" 1.0 1.0 0.0 0 0)
    (Actor|DestroyActor)))

(event EventTick
  (params (DeltaSeconds :type Float%20%28single-precision%29))
  (|CallParentFunction DeltaSeconds) ; 지금 이 노드는 비활성 상태입니다. \n핀을 끌어서 다른 노드를 연결하면 활성화됩니다.
)

(fn ConstructionScript
  (|CallParentFunction))