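; BP_GaruruCanon is a Digimon skill actor that explodes for full radial damage, credited to the player controller.
; It detonates when it overlaps any actor other than the player character, excluding the player from that damage.
; Otherwise it detonates after a short delay from BeginPlay, with no ignore list on that path.
; Both paths spawn an enlarged water-ball hit effect and destroy the actor.
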(event EventBeginPlay
  (bind _returnvalue (Transformation|GetActorLocation))
  (|CallParentFunction)
  (Utilities|FlowControl|Delay 0.8)
  (if true
    (Game|Damage|ApplyRadialDamage (Variables|Default|GetDamage) _returnvalue 1e+03 0 0 self (Game|GetPlayerController 0) true "ECC_WorldDynamic")
    (Effects|SpawnEmitteratLocation "/Game/FXVarietyPack/Particles/P_ky_waterBallHit.P_ky_waterBallHit" _returnvalue "0, 0, 0" "4.000000,4.000000,4.000000")
    (Actor|DestroyActor)))

(event Collision|EventActorBeginOverlap
  (params (OtherActor :type Actor%20Object%20Reference))
  (bind _returnvalue (Transformation|GetActorLocation))
  (bind _returnvalue_2 (Game|GetPlayerCharacter 0))
  (if (!= OtherActor _returnvalue_2)
    (Game|Damage|ApplyRadialDamage (Variables|Default|GetDamage) _returnvalue 1e+03 0 (Utilities|Array|MakeArray _returnvalue_2) self (Game|GetPlayerController 0) true "ECC_WorldDynamic")
    (Effects|SpawnEmitteratLocation "/Game/FXVarietyPack/Particles/P_ky_waterBallHit.P_ky_waterBallHit" _returnvalue "0, 0, 0" "4.000000,4.000000,4.000000")
    (Actor|DestroyActor)))

(event EventTick
  (params (DeltaSeconds :type Float%20%28single-precision%29))
  (|CallParentFunction DeltaSeconds) ; 지금 이 노드는 비활성 상태입니다. \n핀을 끌어서 다른 노드를 연결하면 활성화됩니다.
)

(fn ConstructionScript
  (|CallParentFunction))