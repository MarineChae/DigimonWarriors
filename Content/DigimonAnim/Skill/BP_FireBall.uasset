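; BP_FireBall is a fireball skill actor that explodes when it overlaps an actor tagged Monster.
; On that overlap it applies full radial damage around itself, ignoring player 0's pawn and crediting that player's controller as instigator.
; It then spawns an explosion particle effect and sound at its location and destroys itself.
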(event EventBeginPlay
  (|CallParentFunction) ; 지금 이 노드는 비활성 상태입니다. \n핀을 끌어서 다른 노드를 연결하면 활성화됩니다.
)

(event Collision|EventActorBeginOverlap
  (params (OtherActor :type Actor%20Object%20Reference))
  (bind _returnvalue (Transformation|GetActorLocation))
  (bind _returnvalue_2 (Game|GetPlayerController 0))
  (if (Actor|ActorHasTag OtherActor "Monster")
    (Game|Damage|ApplyRadialDamage (Variables|Default|GetDamage) _returnvalue 5e+02 0 (Utilities|Array|MakeArray (Pawn|GetControlledPawn _returnvalue_2)) self _returnvalue_2 true "ECC_WorldDynamic")
    (Effects|SpawnEmitteratLocation "/Game/MilitaryWeapDark/FX/P_RocketLauncher_Explosion_01.P_RocketLauncher_Explosion_01" _returnvalue "0, 0, 0" "0.500000,0.500000,0.500000")
    (Audio|SpawnSoundatLocation "/Game/Sound/Explosion02.Explosion02" _returnvalue "0, 0, 0" 1.0 1.0 0.0 0 0)
    (Actor|DestroyActor)))

(event EventTick
  (params (DeltaSeconds :type Float%20%28single-precision%29))
  (|CallParentFunction DeltaSeconds) ; 지금 이 노드는 비활성 상태입니다. \n핀을 끌어서 다른 노드를 연결하면 활성화됩니다.
)

(fn ConstructionScript
  (|CallParentFunction))