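; Venom beam skill actor that damages Player-tagged actors overlapping its capsule and spawns a venom explosion effect on them.
; Tick-driven delays toggle capsule collision off and on about every 0.4 seconds, re-triggering overlaps for repeated hits, and destroy the actor after 1.5 seconds.
; An audio component is added on BeginPlay and stopped on EndPlay.
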(event OnComponentBeginOverlap(Capsule)
  (params (OverlappedComponent :type Primitive%20Component%20Object%20Reference) (OtherActor :type Actor%20Object%20Reference) (OtherComp :type Primitive%20Component%20Object%20Reference) (OtherBodyIndex :type Integer) (bFromSweep :type Boolean) (SweepResult :type Hit%20Result%20Structure%20%28by%20ref%29))
  (if (Actor|ActorHasTag OtherActor "Player")
    (Game|Damage|ApplyDamage OtherActor 8e+01 (AI|GetAIController 0) self)
    (Effects|SpawnEmitteratLocation "/Game/DigimonAnim/Skill/VenomExplo.VenomExplo" (Transformation|GetActorLocation OtherActor))))

(event EventBeginPlay
  (bind _returnvalue (AddComponent|AddAudioComponent false))
  (Variables|Default|Setsound _returnvalue))

(event Collision|EventActorBeginOverlap
  (params (OtherActor :type Actor%20Object%20Reference)))

(event EventTick
  (params (DeltaSeconds :type Float%20%28single-precision%29))
  (bind _capsule (Variables|Default|GetCapsule))
  (Utilities|FlowControl|Sequence
    (:then_0
      (Utilities|FlowControl|Delay 0.4)
      (Collision|SetCollisionEnabled _capsule "NoCollision")
      (Collision|SetCollisionEnabled _capsule "QueryAndPhysics"))
    (:then_1
      (Utilities|FlowControl|Delay 1.5)
      (Actor|DestroyActor))))

(event EventEndPlay
  (params (EndPlayReason :type EEndPlayReason%20Enum :default "Destroyed"))
  (Audio|Components|Audio|Stop (Variables|Default|Getsound)))

(fn ConstructionScript)