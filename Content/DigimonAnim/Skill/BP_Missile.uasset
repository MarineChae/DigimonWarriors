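; Homing missile projectile for a player skill, which seeks an enemy and explodes on contact.
; Half a second after spawn it finds the nearest BP_BaseEnemy and switches its ProjectileMovement to home on that actor's root component.
; Overlapping anything except the player character applies full radial damage credited to the player controller, ignoring the player's pawn, then spawns explosion effects and sound and destroys itself.
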(event Custom|SetHomingTarget
  (params (SceneTarget :type Scene%20Component%20Object%20Reference))
  (bind _projectilemovement (Variables|Default|GetProjectileMovement))
  (Utilities|FlowControl|Delay 0.5)
  (bind _outactors (Actor|GetAllActorsOfClass "/Game/DigimonAnim/Enemy/Base/BP_BaseEnemy.BP_BaseEnemy_C"))
  (if (not (Utilities|Array|IsEmpty _outactors))
    (bind _output_get (Variables|Default|SetScene%20Target (Variables|/Script/Engine.Actor|GetRootComponent (.ReturnValue (Actor|FindNearestActor (Transformation|GetActorLocation) _outactors)))))
    (Variables|/Script/Engine.ProjectileMovementComponent|SetbIsHomingProjectile _projectilemovement true)
    (Variables|/Script/Engine.ProjectileMovementComponent|SetHomingAccelerationMagnitude _projectilemovement 7e+03)
    (Variables|/Script/Engine.ProjectileMovementComponent|SetHomingTargetComponent _projectilemovement _output_get)))

(event EventBeginPlay
  (|CallParentFunction)
  (CallFunction|SetHomingTarget))

(event Collision|EventActorBeginOverlap
  (params (OtherActor :type Actor%20Object%20Reference))
  (bind _returnvalue (Transformation|GetActorLocation))
  (bind _returnvalue_2 (Game|GetPlayerController 0))
  (if (!= OtherActor (Game|GetPlayerCharacter 0))
    (Game|Damage|ApplyRadialDamage (Variables|Default|GetDamage) _returnvalue 1e+03 0 (Utilities|Array|MakeArray (Pawn|GetControlledPawn _returnvalue_2)) self _returnvalue_2 true "ECC_WorldDynamic")
    (Effects|SpawnEmitteratLocation "/Game/MilitaryWeapDark/FX/P_RocketLauncher_Explosion_01.P_RocketLauncher_Explosion_01" _returnvalue "0, 0, 0" "1.500000,1.500000,1.500000")
    (Audio|SpawnSoundatLocation "/Game/Sound/Explosion02.Explosion02" _returnvalue "0, 0, 0" 1.0 1.0 0.0 0 0)
    (Actor|DestroyActor)))

(event EventTick
  (params (DeltaSeconds :type Float%20%28single-precision%29)))

(fn ConstructionScript
  (|CallParentFunction))