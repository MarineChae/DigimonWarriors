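; BP_GaiaForce is a Digimon skill actor for the Gaia Force attack, an explosive that grows before it detonates.
; Each Tick multiplies its scale and world Z by small factors until X scale exceeds 2, so growth and height change depend on frame rate.
; Overlapping any actor except player 0's character applies full radial damage that ignores that character, spawns explosion particles and sound, then destroys the actor.
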(event EventBeginPlay
  (|CallParentFunction) ; 지금 이 노드는 비활성 상태입니다. \n핀을 끌어서 다른 노드를 연결하면 활성화됩니다.
)

(event Collision|EventActorBeginOverlap
  (params (OtherActor :type Actor%20Object%20Reference))
  (bind _returnvalue (Transformation|GetActorLocation))
  (bind _returnvalue_2 (Game|GetPlayerCharacter 0))
  (if (!= OtherActor _returnvalue_2)
    (Game|Damage|ApplyRadialDamage (Variables|Default|GetDamage) _returnvalue 3e+03 0 (Utilities|Array|MakeArray _returnvalue_2) self (Game|GetPlayerController 0) true "ECC_WorldDynamic")
    (Effects|SpawnEmitteratLocation "/Game/MilitaryWeapDark/FX/P_RocketLauncher_Explosion_01.P_RocketLauncher_Explosion_01" _returnvalue "0, 0, 0" "5.000000,5.000000,5.000000")
    (Audio|SpawnSoundatLocation "/Game/Sound/Explosion02.Explosion02" _returnvalue "0, 0, 0" 1.0 1.0 0.0 0 0)
    (Actor|DestroyActor)))

(event EventTick
  (params (DeltaSeconds :type Float%20%28single-precision%29))
  (bind _returnvalue (Transformation|GetActorLocation))
  (|CallParentFunction DeltaSeconds)
  (if (not (< 2.0 (.x (Transformation|GetActorScale3D))))
    (Transformation|SetActorScale3D (* (Transformation|GetActorScale3D) 1.013))
    (Transformation|SetActorLocation (Math|Vector|MakeVector (.x _returnvalue) (.y _returnvalue) (* (.z _returnvalue) 1.002)) false false)))

(fn ConstructionScript
  (|CallParentFunction))